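; Monster enemy Blueprint that chases the player on sight, attacks in melee and reacts to hits.
; PawnSensing starts an AI MoveTo toward the player, triggering Attack within range, with CanAttack locking it during a delayed cooldown.
; Attack snaps rotation toward the first agent overlapping the Box before playing its montage.
; TakeDamage forwards hits to the BP_ZZZ_CharacterBase hit event, then plays a hit reaction or a death montage followed by destruction.
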(event `self.ReceiveBeginPlay`
  (set `self.DodgeBox` (`self.Box`)))

(event `Attack`
  ; 공격
  (if (`self.CanAttack`)
    (`self.AutoTargeting` self)
    (`self.PlayAnimMontage` self "/Game/Monster/MBP_MonsterAttackMontague.MBP_MonsterAttackMontague" 1.0 "MonsterCombo1")
    ;; 공격 쿨타임
    (`KismetSystemLibrary.Delay` 3.0)
    (set `self.CanAttack` false)))

(event `self.PawnSensing.OnSeePawn`
  (params (Pawn :type "Pawn Object Reference"))
  ; 몬스터 시야각에 플레이어 감지시 실행
  (if (not (`self.IsDead`))
    (set `self.DetetecedPlayer` (`KismetSystemLibrary.IsValid` Pawn))
    (`self.FollowPlayer`)))

(event `FollowPlayer`
  (bind _returnvalue (`self.GetDistanceTo` self (`GameplayStatics.GetPlayerPawn` 0)))
  ; FollowPlayer
  (if (`self.DetetecedPlayer`)
    (`|AIMoveTo` self (0.0 0.0 0.0) (`GameplayStatics.GetPlayerCharacter` 0) 30.0 true
      (:`then`
        ;; 거리 체크로 공격할지 말지 결정
        (if (and (<= _returnvalue 200.0) (!= (`self.CanAttack`) true))
          (`KismetSystemLibrary.PrintString` (`KismetStringLibrary.Conv_DoubleToString` _returnvalue))
          (set `self.CanAttack` true)
          (`self.Attack`))))))

(event `Death`
  ; 죽음
  (`self.PlayAnimMontage` "/Game/Monster/Mon_MonsterDeath.Mon_MonsterDeath" 1.0 "MonsterDie")
  (`KismetSystemLibrary.Delay` 1.9)
  (`self.K2_DestroyActor`))

(fn `AutoTargeting`
  (bind _overlappingactors (`PrimitiveComponent.GetOverlappingActors` (`self.Box`) "/Game/Blueprints/BP_ZZZ_AgentBase.BP_ZZZ_AgentBase_C"))
  ; 오토 타겟팅 시스템
  (if (`KismetArrayLibrary.Array_IsNotEmpty` _overlappingactors)
    (`self.K2_SetActorRotation` (`KismetMathLibrary.FindLookAtRotation` (`self.K2_GetActorLocation` (`self.GetOwner`)) (`self.K2_GetActorLocation` (`|GetArrayItem` _overlappingactors))))))

(fn `TakeDamage`
  (params (Damage :type "Float (double-precision)") (Target :type "Actor Object Reference"))
  (locals (NewLocalVar :type "Actor Object Reference"))
  (`KismetSystemLibrary.PrintString` "Hello")
  (bind _asbp_zzz_character_base (cast `/Game/Blueprints/BP_ZZZ_CharacterBase` self))
  ; 01. 죽었는지 검사
  (set `self.Target` null)
  (if (not (`/Game/Blueprints/BP_ZZZ_CharacterBase.IsDead?` _asbp_zzz_character_base))
    (bind _asbp_zzz_character_base_2 (cast `/Game/Blueprints/BP_ZZZ_CharacterBase` self))
    (`self.OnCharacterHItEvent` _asbp_zzz_character_base_2 (`local.Target`))
    (if (`/Game/Blueprints/BP_ZZZ_CharacterBase.IsDead?` _asbp_zzz_character_base_2)
      (`self.Death` self)
      (else
        (`self.PlayAnimMontage` "/Game/Monster/Mon_MonsterHit.Mon_MonsterHit")))))

(fn `UserConstructionScript`)