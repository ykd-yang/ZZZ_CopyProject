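; Base enemy Blueprint that targets the player pawn, cached on BeginPlay as a BP_ZZZ_AgentBase.
; Offers helpers to move straight toward the player by setting location without sweep and snap yaw to face them.
; Range checks cover a dot-product view test (converted via R2D without Acos) and charge-attack distance; the normal-attack check always returns false.
; Attack warnings spawn a scaled Niagara effect attached to the mesh at AttackSocket's location.
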(event `self.ReceiveBeginPlay`
  ; 공격 목표인 플레이어
  (bind _asbp_zzz_agent_base (cast `/Game/Blueprint/BP_ZZZ_AgentBase` (`GameplayStatics.GetPlayerPawn` 0))
    (:`then`
      (set `self.Player` _asbp_zzz_agent_base))
    (:`CastFailed`
      (`KismetSystemLibrary.PrintString` "웁스"))))

(fn `CheckPlayerInChargeAttackRange`
  (returns (`In ChargeAttackRange` :type Boolean))
  (return (<= (`KismetMathLibrary.Vector_Distance` (`self.K2_GetActorLocation` (`self.Player`)) (`self.K2_GetActorLocation` self)) (`self.ChargeAttackRange`))))

(fn `CheckPlayerInFieldOfView`
  (returns (`In FieldOfView` :type Boolean))
  (return (<= (`KismetMathLibrary.RadiansToDegrees` (`KismetMathLibrary.Dot_VectorVector` (`KismetMathLibrary.Normal` (- (`self.K2_GetActorLocation` (`self.Player`)) (`self.K2_GetActorLocation` self))) (`KismetMathLibrary.Normal` (`self.GetActorForwardVector` self)))) (`self.FieldOfView`))))

(fn `CheckPlayerInNormalAttackRange`
  (returns (`Player In Attack Range` :type Boolean))
  (return false))

(fn `PlayAttackWarning`
  (params (NiagaraSystem :type "NiagaraSystem Object Reference") (Scale :type "Float (double-precision)"))
  (bind _mesh_comp (`self.GetMesh`))
  (if (`KismetSystemLibrary.IsValid` NiagaraSystem)
    (bind _returnvalue (`NiagaraFunctionLibrary.SpawnSystemAttached` NiagaraSystem _mesh_comp "None" (`SceneComponent.GetSocketLocation` _mesh_comp "AttackSocket") (struct) "KeepWorldPosition" true true "AutoRelease"))
    (`SceneComponent.SetWorldScale3D` _returnvalue (`KismetMathLibrary.Conv_DoubleToVector` Scale))))

(fn `Turn`
  (bind (_returnvalue_x _returnvalue_y) (`KismetMathLibrary.BreakVector` (- (`self.K2_GetActorLocation` (`self.Player`)) (`self.K2_GetActorLocation`))))
  (`self.K2_SetActorRotation` (`KismetMathLibrary.MakeRotator` 0.0 0.0 (`KismetMathLibrary.RadiansToDegrees` (`KismetMathLibrary.Atan2` _returnvalue_y _returnvalue_x)))))

(fn `UserConstructionScript`
  (`parent.UserConstructionScript`))

(fn `Walk`
  (`self.K2_SetActorLocation` (+ (* (`KismetMathLibrary.Normal` (- (`self.K2_GetActorLocation` (`self.Player`)) (`self.K2_GetActorLocation`))) (`self.Speed`) (`GameplayStatics.GetWorldDeltaSeconds`)) (`self.K2_GetActorLocation`)))
  (return))