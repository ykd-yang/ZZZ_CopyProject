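; BP_ZZZ_CharacterBase is a base character Blueprint that handles hit damage and death.
; OnCharacterHItEvent requires a living character as the hit source, then reduces its ATK by this character's DEF percentage, clamps HP and calls death or hit feedback.
; The IFF switch has empty branches.
; A second sequence branch subtracts trap DMG without a death check, behind the same character cast, so it needs a source passing both casts.
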(event Custom|OnCharacterHItEvent
  (params (other :type Actor%20Object%20Reference))
  (bind _self self)
  (bind _asbp_zzz_character_base (Utilities|Casting|CastToBP_ZZZ_CharacterBase other))
  (if (not (Variables|BP_ZZZ_CharacterBase_C|GetIsDead? _asbp_zzz_character_base))
    (Utilities|FlowControl|Sequence
      (:then_0
        ;[0.15 0.15 0.15 0.5] 공격 유형을 확인한 후 데미지 적용
        (bind _asbp_zzz_character_base_2 (Utilities|Casting|CastToBP_ZZZ_CharacterBase other))
        (switch Utilities|FlowControl|Switch|SwitchonTeamType (Variables|BP_ZZZ_CharacterBase_C|GetIFF _asbp_zzz_character_base_2)
          (:NewEnumerator0
            _)
          (:NewEnumerator1
            _)
          (:NewEnumerator2
            _))
        (bind _output_get (Variables|Default|SetHP (Math|Float|Truncate (Math|Float|Clamp(Float) (- (Variables|Default|GetHP) (|(((100-defend)/100)*attack) (Math|Conversions|ToFloat(Integer) (Variables|Default|GetDEF)) (Math|Conversions|ToFloat(Integer) (Variables|BP_ZZZ_CharacterBase_C|GetATK _asbp_zzz_character_base_2)))) 0.0 1e+05))))
        (bind _output_get_2 (Variables|Default|SetIsDead? (<= _output_get 0)))
        (if _output_get_2
          (Class|BPIBehaivour|PlayDeath(Message) _self)
          (else
            (Class|BPIBehaivour|GetHit(Message) _self))))
      (:then_1
        ;[0.15 0.15 0.15 0.5] 함정 데미지 적용
        (bind _asbp_zzz_trap_base (Utilities|Casting|CastToBP_ZZZ_TrapBase other))
        (Variables|Default|SetHP (Math|Float|Truncate (Math|Float|Clamp(Float) (Math|Conversions|ToFloat(Integer) (- (Variables|Default|GetHP) (Variables|/Game/Blueprint/BP_ZZZ_TrapBase.BP_ZZZ_TrapBase_C|GetDMG _asbp_zzz_trap_base))) 0.0 1e+05)))
        (Development|PrintString "AgentDamaged")))))

(fn ConstructionScript)