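; BP_StageManager tracks kills and advances the game through up to three stages.
; BeginPlay loads the first stage's row from a data table.
; AddKill prints the kill count and calls ClearStage when it reaches that row's monster count.
; ClearStage resets kills, calls WhenClear on the current stage's enemy spawner to open the next stage, then loads the next row or prints the stage number past the last.
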(event `self.ReceiveBeginPlay`
  (bind _returnvalue (`|GetDataTableRow` "/Game/Blueprint/Spawner/StageTableDatas.StageTableDatas" "1")
    (:`then`
      (set `self.CurrentStageInfo` _returnvalue))))

(fn `AddKill`
  (bind (_currentstageinfo_bossstage_ _currentstageinfo_stagenumber `_currentstageinfo_그스테이지에서소환되어야하는몬스터수`) (break `/Game/Blueprint/Spawner/StageTable` (`self.CurrentStageInfo`)))
  (bind _returnvalue (+ (`self.CurrentKill`) 1))
  (set `self.CurrentKill` _returnvalue)
  (if (>= _returnvalue `_currentstageinfo_그스테이지에서소환되어야하는몬스터수`)
    (`KismetSystemLibrary.PrintString` (`KismetStringLibrary.Concat_StrStr` (`KismetStringLibrary.Conv_IntToString` (`self.CurrentKill`)) "킬"))
    (`self.ClearStage`)
    (else
      (`KismetSystemLibrary.PrintString` (`KismetStringLibrary.Concat_StrStr` (`KismetStringLibrary.Conv_IntToString` (`self.CurrentKill`)) "킬")))))

(fn `ClearStage`
  (bind _output (`|GetArrayItem` (`self.EnemySpawners`) (- (`self.CurrentStage`) 1)))
  (set `self.CurrentKill` 0)
  ; 다음 스테이지 개방
  (if (`KismetSystemLibrary.IsValid` _output)
    (`/Game/Blueprint/Spawner/BP_EnemySpawner.WhenClear` _output)
    (bind _result (`/Engine/EditorBlueprintResources/StandardMacros.IncrementInt` (`self.CurrentStage`))
      (:`  `
        (if (<= _result 3)
          (bind _returnvalue (`KismetStringLibrary.Conv_StringToName` (`KismetStringLibrary.Conv_IntToString` _result)))
          (bind _returnvalue_2 (`|GetDataTableRow` "/Game/Blueprint/Spawner/StageTableDatas.StageTableDatas" _returnvalue)
            (:`then`
              (set `self.CurrentStageInfo` _returnvalue_2)))
          (else
            (`KismetSystemLibrary.PrintString` (`KismetStringLibrary.Concat_StrStr` "다음스테이지는" (`KismetStringLibrary.Conv_NameToString` _returnvalue)))))))))

(fn `UserConstructionScript`)