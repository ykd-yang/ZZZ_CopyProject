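; BP_EnemySpawner is a one-time enemy spawner that fills a stage with Claymore monsters or bosses when the spawn trigger box fires.
; It reads monster count and boss flag from the StageManager's current stage info, then spawns actors in a row along Y.
; Claymore death signals feed kills back to the StageManager; boss deaths are not counted here.
; A separate WhenClear event destroys the Barrier behind a DoOnce.
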(event `SpawnEnemy`
  (bind (_currentstageinfo_bossstage_ _currentstageinfo_stagenumber `_currentstageinfo_그스테이지에서소환되어야하는몬스터수`) (break `/Game/Blueprint/Spawner/StageTable` (`/Game/Blueprint/Spawner/BP_StageManager.CurrentStageInfo` (`self.StageManager`))))
  (if (not (`self.EndSpawn`))
    (for _index (range `_currentstageinfo_그스테이지에서소환되어야하는몬스터수`)
      (if _currentstageinfo_bossstage_
        (bind _returnvalue (+ (`self.K2_GetActorLocation`) (`KismetMathLibrary.MakeVector` 0.0 (* _index 200))))
        (bind _returnvalue_2 (`|SpawnActorFromClass` "/Game/Enemy/ModifiedDurahan/Blueprint/BP_Boss.BP_Boss_C" (`KismetMathLibrary.MakeTransform` _returnvalue) "AlwaysSpawn" "MultiplyWithRoot" null null))
        (bind _asbp_boss (cast `/Game/Enemy/ModifiedDurahan/Blueprint/BP_Boss` _returnvalue_2))
        (if (`KismetSystemLibrary.IsValid` _asbp_boss)
          (`/Engine/EditorBlueprintResources/StandardMacros.DoOnce` false))
        (else
          (bind _returnvalue_3 (`|SpawnActorFromClass` "/Game/Enemy/ModifiedClaymore/Blueprint/BP_Claymore.BP_Claymore_C" (`KismetMathLibrary.MakeTransform` _returnvalue) "AlwaysSpawn" "MultiplyWithRoot" null null))
          (bind _asbp_claymore (cast `/Game/Enemy/ModifiedClaymore/Blueprint/BP_Claymore` _returnvalue_3))
          (if (`KismetSystemLibrary.IsValid` _asbp_claymore)
            (add `/Game/Blueprint/BP_ZZZ_EnemyBase.DeadSignal` _asbp_claymore (delegate `AddKillCount`))))))
    (set `self.EndSpawn` true)))

(event `AddKillCount`
  (bind _returnvalue (`GameplayStatics.GetActorOfClass` "/Game/Blueprint/Spawner/BP_StageManager.BP_StageManager_C"))
  (`/Game/Blueprint/Spawner/BP_StageManager.AddKill` _returnvalue))

(event `self.ReceiveBeginPlay`
  (bind _returnvalue (`GameplayStatics.GetActorOfClass` "/Game/Blueprint/Spawner/BP_StageManager.BP_StageManager_C"))
  (set `self.StageManager` _returnvalue)
  (bind _returnvalue_2 (`GameplayStatics.GetActorOfClass` "/Game/Blueprint/Spawner/BP_SpawnTriggerBox.BP_SpawnTriggerBox_C"))
  (add `/Game/Blueprint/Spawner/BP_SpawnTriggerBox.CanSpawn!` _returnvalue_2 (delegate `SpawnEnemy`)))

(event `WhenClear`
  (`/Engine/EditorBlueprintResources/StandardMacros.DoOnce` false
    (:`Completed`
      (`self.K2_DestroyActor` (`self.Barrier`)))))

(fn `UserConstructionScript`)