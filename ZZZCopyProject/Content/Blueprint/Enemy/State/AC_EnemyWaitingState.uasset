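; Enemy state component that holds a BP_Enemy in a brief waiting pause before it returns to idle.
; BeginPlay caches the owning enemy.
; Enter clears the walking flag and starts a one-second timer that switches the enemy's state machine component to its idle state.
; Exit and Update are empty, and the timer is not cleared on exit.
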(event `self.ReceiveBeginPlay`
  (bind _asbp_enemy (cast `/Game/Blueprint/Enemy/State/BP_Enemy` (`self.GetOwner`)))
  (set `self.OwnerEnemy` _asbp_enemy))

(event `self.Exit`)

(event `self.Update`)

(event `self.Enter`
  (set `/Game/Blueprint/Enemy/State/BP_Enemy.isWalking?` false (`self.OwnerEnemy`))
  (`KismetSystemLibrary.K2_SetTimerDelegate` (delegate `ToIdle`) 1.0))

(event `ToIdle`
  (bind _ownerenemy (`self.OwnerEnemy`))
  (`/Game/Blueprint/Interface/BPI_IEnemyStateMachine.ChangeState` (`/Game/Blueprint/Enemy/State/BP_Enemy.AC_EnemyStateMachine` _ownerenemy) (`/Game/Blueprint/Enemy/State/BP_Enemy.AC_EnemyIdleState` _ownerenemy)))