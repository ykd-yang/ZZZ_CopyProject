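; Actor component implementing the walk state of an enemy's state machine on BP_Enemy.
; It caches the owning enemy on BeginPlay and toggles its IsWalking flag on Enter and Exit.
; Each Update turns and walks the enemy until its player distance check returns true, then switches the state machine to the idle state.
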(event `self.ReceiveBeginPlay`
  (bind _asbp_enemy (cast `/Game/Blueprint/Enemy/State/BP_Enemy` (`self.GetOwner`)))
  (set `self.OwnerEnemy` _asbp_enemy))

(event `self.Enter`
  (set `/Game/Blueprint/Enemy/State/BP_Enemy.isWalking?` true (`self.OwnerEnemy`)))

(event `self.Update`
  (bind _ownerenemy (`self.OwnerEnemy`))
  (bind _canattackdistance (`/Game/Blueprint/Enemy/State/BP_Enemy.CheckDistanceWithPlayer` _ownerenemy))
  (if _canattackdistance
    (`/Game/Blueprint/Interface/BPI_IEnemyStateMachine.ChangeState` (`/Game/Blueprint/Enemy/State/BP_Enemy.AC_EnemyStateMachine` _ownerenemy) (`/Game/Blueprint/Enemy/State/BP_Enemy.AC_EnemyIdleState` _ownerenemy))
    (else
      (`/Game/Blueprint/Enemy/State/BP_Enemy.Turn` _ownerenemy)
      (`/Game/Blueprint/Enemy/State/BP_Enemy.Walking` _ownerenemy))))

(event `self.Exit`
  (set `/Game/Blueprint/Enemy/State/BP_Enemy.isWalking?` false (`self.OwnerEnemy`)))