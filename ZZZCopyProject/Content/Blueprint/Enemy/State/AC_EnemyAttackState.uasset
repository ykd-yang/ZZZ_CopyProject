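; Enemy attack state component for BP_Enemy, used by its enemy state machine to perform an attack.
; BeginPlay caches the owning BP_Enemy.
; Enter calls the enemy's attack targeting, then plays the attack montage on its mesh and switches the state machine to idle when the montage completes.
; Update and Exit are empty.
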(event `self.ReceiveBeginPlay`
  (bind _asbp_enemy (cast `/Game/Blueprint/Enemy/State/BP_Enemy` (`self.GetOwner`)))
  (set `self.OwnerEnemy` _asbp_enemy))

(event `self.Enter`
  (bind _ownerenemy (`self.OwnerEnemy`))
  (`/Game/Blueprint/Enemy/State/BP_Enemy.AttackTargeting` _ownerenemy)
  (`|PlayMontage` (`Character.Mesh` _ownerenemy) "/Game/Enemy/ModifiedClaymore/Animation/Montage/AM_EnemyAttack.AM_EnemyAttack"
    (:`OnCompleted`
      (`/Game/Blueprint/Interface/BPI_IEnemyStateMachine.ChangeState` (`/Game/Blueprint/Enemy/State/BP_Enemy.AC_EnemyStateMachine` _ownerenemy) (`/Game/Blueprint/Enemy/State/BP_Enemy.AC_EnemyIdleState` _ownerenemy)))))

(event `self.Update`)

(event `self.Exit`)