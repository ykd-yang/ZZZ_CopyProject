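; Anim notify state that marks the dodge window within an agent's animation.
; On begin it casts the mesh owner to BP_ZZZ_AgentBase and sets IsOnDodging true; on end it sets the flag false.
; Both events print a debug string, and owners of any other class are ignored.
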(fn `Received_NotifyBegin`
  (params (MeshComp :type "SkeletalMeshComponent Object Reference") (Animation :type "AnimSequenceBase Object Reference") (TotalDuration :type "Float (single-precision)") (EventReference :type "AnimNotifyEventReference Structure (by ref)"))
  (returns (ReturnValue :type Boolean))
  (bind _asbp_zzz_agent_base (cast `/Game/Blueprint/BP_ZZZ_AgentBase` (`ActorComponent.GetOwner` MeshComp)))
  (set `/Game/Blueprint/BP_ZZZ_AgentBase.IsOnDodging` true _asbp_zzz_agent_base)
  (`KismetSystemLibrary.PrintString` null "Start")
  (return false))

(fn `Received_NotifyEnd`
  (params (MeshComp :type "SkeletalMeshComponent Object Reference") (Animation :type "AnimSequenceBase Object Reference") (EventReference :type "AnimNotifyEventReference Structure (by ref)"))
  (returns (ReturnValue :type Boolean))
  (bind _asbp_zzz_agent_base (cast `/Game/Blueprint/BP_ZZZ_AgentBase` (`ActorComponent.GetOwner` MeshComp)))
  (set `/Game/Blueprint/BP_ZZZ_AgentBase.IsOnDodging` false _asbp_zzz_agent_base)
  (`KismetSystemLibrary.PrintString` null "End")
  (return false))