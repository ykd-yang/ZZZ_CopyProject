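; BP_ZZZ_AgentBase is a base character Blueprint for playable agents, handling movement states, hit response and skill input.
; Tick derives moving state from velocity, shifts into a faster run after a timed delay, and computes a signed body shear from facing versus velocity.
; Hits register as successful dodges while dodging; otherwise they forward to hit handling and a dispatcher.
; E triggers skills; right-click dodge logic sits behind an always-false condition.
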(event `OnAgentHitEvent`
  (params (other :type "/Game/Blueprint/BP_ZZZ_CharacterBase Object Reference"))
  ; 플레이어 피격 이벤트 => 회피중인 확인 - 아니라면 데미지 입음 + 회피 실패 , 맞다면 No 데미지 +
  (if (`self.IsOnDodging`)
    (set `self.DodgingSuccess` true)
    (else
      (`self.OnCharacterHItEvent` other)
      (set `self.DodgingSuccess` false)
      (`self.OnHitEventDispatcher`))))

(event `self.ReceiveTick`
  (params (DeltaSeconds :type "Float (single-precision)"))
  (bind _returnvalue (`self.GetActorForwardVector`))
  (bind _returnvalue_2 (`KismetMathLibrary.Normal` (`MovementComponent.Velocity` (`self.CharacterMovement`))))
  (`|ExecutionSequence`
    (:`then_0`
      ; 캐릭터 무브 컴포넌트를 사용하여 이동 상태를 확인 - 이동 상태로 전환하거나 정지 상태로 전환한다
      (if (> (`KismetMathLibrary.VSize` (`MovementComponent.Velocity` (`self.CharacterMovement`))) 50.0)
        (set `self.IsMoving` true)
        (else
          (set `self.IsMoving` false)
          (set `self.IsRunning` false)
          ;; 이동 속도 감소 및 달리기 전환 타이머 비활성
          (set `CharacterMovementComponent.MaxWalkSpeed` 600.0 (`self.CharacterMovement`))
          (`KismetSystemLibrary.K2_ClearAndInvalidateTimerHandle` (`self.RunningTransitionTimerHandle`)))))
    (:`then_1`
      ; Comment
      ;; 이동 상태인데 아직 달리는 상태는 아닌가 확인
      (if (and (`self.IsMoving`) (not (`self.IsRunning`)))
        ;; 달리기 시작 타이머 시작한다
        (if (not (`KismetSystemLibrary.K2_IsValidTimerHandle` (`self.RunningTransitionTimerHandle`)))
          (bind _returnvalue_3 (`KismetSystemLibrary.K2_SetTimerDelegate` (delegate `EnterRunningState`) 2.0))
          (set `self.RunningTransitionTimerHandle` _returnvalue_3)
          (`KismetSystemLibrary.PrintString` "Running Timer Start" true true (struct :`G` 1.0 :`A` 1.0)))))
    (:`then_2`
      ; Comment
      (set `self.BodyShearRate` (* (- (`KismetMathLibrary.Dot_VectorVector` _returnvalue _returnvalue_2) 1.0) 600.0 (`KismetMathLibrary.SignOfFloat` (`KismetMathLibrary.CrossProduct2D` (`KismetMathLibrary.Conv_VectorToVector2D` _returnvalue) (`KismetMathLibrary.Conv_VectorToVector2D` _returnvalue_2))))))))

(event `EnterRunningState`
  ; Comment
  ;; 달리기 시작 타이머가 발동 되면 이동 속도 증가
  (`KismetSystemLibrary.PrintString` "Enter Running State" true true (struct :`G` 1.0 :`A` 1.0))
  (set `self.IsRunning` true)
  (set `CharacterMovementComponent.MaxWalkSpeed` 900.0 (`self.CharacterMovement`))
  (`KismetSystemLibrary.K2_ClearAndInvalidateTimerHandle` (`self.RunningTransitionTimerHandle`)))

(event `Key|RightMouseButton`
  (params (Key :type "Key Structure"))
  (bind _returnvalue (<= (`KismetMathLibrary.Dot_VectorVector` (`self.GetVelocity`) (`self.GetActorForwardVector`)) 200.0))
  ; 우클릭 회피 로직
  (:`Pressed`
    (if (>= 0 1)
      (set `self.IsRightMouseDown` true)
      (set `CharacterMovementComponent.MaxWalkSpeed` 1800.0 (`self.CharacterMovement`))
      (set `MovementComponent.Velocity` (* (`self.GetActorForwardVector`) (`KismetMathLibrary.SelectInt` -1800 1800 _returnvalue)) (`self.CharacterMovement`))
      (`KismetSystemLibrary.K2_SetTimerDelegate` (delegate `DodgeOverEvent`) 0.4)
      (`|ExecutionSequence`
        (:`then_0`
          (`/Game/Blueprint/Interface/BPI_Dodge.DodgePlay` _returnvalue)))))
  (:`Released`
    (set `self.IsRightMouseDown` false)))

(event `DodgeOverEvent`
  ; 회피 종료
  (set `CharacterMovementComponent.MaxWalkSpeed` 600.0 (`self.CharacterMovement`)))

(event `Key|E`
  (params (Key :type "Key Structure"))
  (:`Pressed`
    (message `/Game/Blueprint/Interface/BPI_Skill.ExecuteSkill` self)))

(event `/Game/Blueprint/Interface/Behivour/BPI_Common_Behaviour.Damaged`
  (params (KnockBack :type "Vector Structure") (Damage :type Integer) (HitParticle :type "NiagaraComponent Object Reference") (HitParticleScale :type "Float (double-precision)")))

(fn `UserConstructionScript`)