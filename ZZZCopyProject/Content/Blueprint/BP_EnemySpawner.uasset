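; BP_EnemySpawner is an actor that brings enemies into play when dialogue ends.
; On BeginPlay it binds to the BP_ZZZ_GameMode dialogue-end dispatcher, choosing the boss or regular handler by the EnemyBoss flag.
; The regular handler spawns a BP_Claymore at the spawner's transform and sets its EndSpawn flag after a short delay.
; The boss handler spawns nothing, instead setting EndSpawn on the BP_Boss already in the level.
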(event `self.ReceiveBeginPlay`
  (bind _asbp_zzz_game_mode (cast `/Game/Blueprint/BP_ZZZ_GameMode` (`GameplayStatics.GetGameMode`)))
  (if (`self.Enemy?Boss?`)
    (add `/Game/Blueprint/BP_ZZZ_GameMode.OnDialogueEnd_Dispatcher` _asbp_zzz_game_mode (delegate `BossSpawnEvent`))
    (else
      (add `/Game/Blueprint/BP_ZZZ_GameMode.OnDialogueEnd_Dispatcher` _asbp_zzz_game_mode (delegate `EnemySpawner`)))))

(event `EnemySpawner`
  (bind _returnvalue (`|SpawnActorFromClass` "/Game/Blueprint/Claymore/State/BP_Claymore.BP_Claymore_C" (`self.GetTransform` self) "Undefined" "MultiplyWithRoot" null null))
  (bind _asbp_enemy (cast `/Game/Blueprint/Claymore/State/BP_Claymore` _returnvalue))
  (`KismetSystemLibrary.Delay` 1.0)
  (set `/Game/Blueprint/Claymore/State/BP_Claymore.EndSpawn` true _asbp_enemy))

(event `BossSpawnEvent`
  (bind _returnvalue (`GameplayStatics.GetActorOfClass` "/Game/Blueprint/Boss/BP_Boss.BP_Boss_C"))
  (bind _asbp_boss (cast `/Game/Blueprint/Boss/BP_Boss` _returnvalue))
  (set `/Game/Blueprint/Boss/BP_Boss.EndSpawn` true _asbp_boss))

(fn `UserConstructionScript`)