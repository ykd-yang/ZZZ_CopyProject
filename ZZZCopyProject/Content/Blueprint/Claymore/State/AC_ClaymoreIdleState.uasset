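; Idle state component for the Claymore enemy, run by its state machine.
; On BeginPlay it caches the owning BP_Claymore, and entering the state clears the walking flag.
; Each update immediately switches to the attack state when the player is within normal attack range, otherwise to the walk state.
; Exiting prints a debug message.
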(event `self.ReceiveBeginPlay`
  ; Comment
  (bind _asbp_claymore (cast `/Game/Blueprint/Claymore/State/BP_Claymore` (`self.GetOwner`)))
  (set `self.OwnerEnemy` _asbp_claymore))

(event `/Game/Blueprint/Interface/BPI_IEnemyState.Enter`
  ; Comment
  (set `/Game/Blueprint/Claymore/State/BP_Claymore.isWalking?` false (`self.OwnerEnemy`)))

(event `/Game/Blueprint/Interface/BPI_IEnemyState.Update`
  (bind _ownerenemy (`self.OwnerEnemy`))
  (bind _ownerenemy_2 (`self.OwnerEnemy`))
  (if (`/Game/Blueprint/BP_ZZZ_EnemyBase.CheckPlayerInNormalAttackRange` (`self.OwnerEnemy`))
    ; Comment
    (`/Game/Blueprint/Interface/BPI_IEnemyStateMachine.ChangeState` (`/Game/Blueprint/Claymore/State/BP_Claymore.AC_ClaymoreStateMachine` _ownerenemy_2) (`/Game/Blueprint/Claymore/State/BP_Claymore.AC_ClaymoreAttackState` _ownerenemy_2))
    (else
      ; Comment
      (`/Game/Blueprint/Interface/BPI_IEnemyStateMachine.ChangeState` (`/Game/Blueprint/Claymore/State/BP_Claymore.AC_ClaymoreStateMachine` _ownerenemy) (`/Game/Blueprint/Claymore/State/BP_Claymore.AC_ClaymoreWalkState` _ownerenemy)))))

(event `/Game/Blueprint/Interface/BPI_IEnemyState.Exit`
  (`KismetSystemLibrary.PrintString` "아이들 나감"))