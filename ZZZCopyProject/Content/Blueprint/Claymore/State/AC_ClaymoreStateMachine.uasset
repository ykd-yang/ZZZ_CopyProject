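; State machine component for the Claymore enemy, BP_Claymore, that switches between and runs its behavior states.
; States are used through an interface: ChangeState exits the current one, records it as previous and enters the requested one, unless the owner is dead.
; With no valid current state, ChangeState ignores the request and enters the owner's Idle state.
; Execute forwards updates to the current state.
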(event `self.ReceiveBeginPlay`
  ; Comment
  (bind _asbp_claymore (cast `/Game/Blueprint/Claymore/State/BP_Claymore` (`self.GetOwner`)))
  (set `self.OwnerEnemy` _asbp_claymore)
  (`KismetSystemLibrary.PrintString` (`KismetStringLibrary.Concat_StrStr` (`KismetSystemLibrary.GetDisplayName` _asbp_claymore) "'s State Machine is Ready!") true true (struct :`R` 1.0 :`A` 1.0)))

(event `/Game/Blueprint/Interface/BPI_IEnemyStateMachine.ChangeState`
  (params (ChangeEnemyState :type "/Game/Blueprint/Interface/BPI_IEnemyState Interface"))
  (bind _currentstate (`self.CurrentState`))
  (if (not (`/Game/Blueprint/BP_ZZZ_CharacterBase.Dead?` (`self.OwnerEnemy`)))
    (if (`KismetSystemLibrary.IsValidInterface` (`self.CurrentState`))
      ; Comment
      (`/Game/Blueprint/Interface/BPI_IEnemyState.Exit` _currentstate)
      (set `self.PreviousState` _currentstate)
      (bind _output_get (set `self.CurrentState` ChangeEnemyState))
      (`/Game/Blueprint/Interface/BPI_IEnemyState.Enter` _output_get)
      (else
        ; 최초 실행
        (bind _output_get_2 (set `self.CurrentState` (`/Game/Blueprint/Claymore/State/BP_Claymore.AC_ClaymoreIdleState` (`self.OwnerEnemy`))))
        (bind _output_get_3 (set `self.PreviousState` _output_get_2))
        (`/Game/Blueprint/Interface/BPI_IEnemyState.Enter` _output_get_3)))))

(event `/Game/Blueprint/Interface/BPI_IEnemyStateMachine.Execute`
  (bind _currentstate (`self.CurrentState`))
  ; Comment
  (if (`KismetSystemLibrary.IsValidInterface` _currentstate)
    (`/Game/Blueprint/Interface/BPI_IEnemyState.Update` _currentstate)))