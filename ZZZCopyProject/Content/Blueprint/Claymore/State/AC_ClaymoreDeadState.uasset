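; AC_ClaymoreDeadState is the death state component for the Claymore enemy, caching its BP_Claymore owner on BeginPlay.
; On Enter it flags the owner dead, starts the death montage and immediately sets the capsule to ignore the Pawn channel.
; After a fixed delay, rather than on montage completion, it adds to the kill count on BP_AlphaManager and destroys the enemy.
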(event `self.ReceiveBeginPlay`
  ; Comment
  (bind _asbp_claymore (cast `/Game/Blueprint/Claymore/State/BP_Claymore` (`self.GetOwner`)))
  (set `self.OwnerEnemy` _asbp_claymore))

(event `/Game/Blueprint/Interface/BPI_IEnemyState.Enter`
  (bind _ownerenemy (`self.OwnerEnemy`))
  (set `/Game/Blueprint/BP_ZZZ_CharacterBase.Dead?` true _ownerenemy)
  (`|PlayMontage` (`Character.Mesh` _ownerenemy) "/Game/Enemy/ModifiedClaymore/Animation/Montage/AM_EnemyDie.AM_EnemyDie"
    (:`then`
      (`PrimitiveComponent.SetCollisionResponseToChannel` (`Character.CapsuleComponent` (`self.OwnerEnemy`)) "ECC_Pawn" "ECR_Ignore")
      (`KismetSystemLibrary.Delay` 5.0)
      (bind _returnvalue (`GameplayStatics.GetActorOfClass` "/Game/Blueprint/BP_AlphaManager.BP_AlphaManager_C"))
      (`/Game/Blueprint/BP_AlphaManager.AddKillCount` _returnvalue)
      (`Actor.K2_DestroyActor` (`self.OwnerEnemy`)))))