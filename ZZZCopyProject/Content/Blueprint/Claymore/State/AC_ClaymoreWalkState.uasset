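; AC_ClaymoreWalkState is the walk state component for the Claymore enemy's component-based state machine.
; It caches its BP_Claymore owner on BeginPlay and toggles the owner's IsWalking flag on Enter and Exit.
; Each Update turns and walks the enemy until the player is in normal attack range, then switches the state machine to the idle state.
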(event `self.ReceiveBeginPlay`
  ; Comment
  (bind _asbp_claymore (cast `/Game/Blueprint/Claymore/State/BP_Claymore` (`self.GetOwner`)))
  (set `self.OwnerEnemy` _asbp_claymore))

(event `self.Enter`
  ; Comment
  (set `/Game/Blueprint/Claymore/State/BP_Claymore.isWalking?` true (`self.OwnerEnemy`)))

(event `self.Update`
  (bind _ownerenemy (`self.OwnerEnemy`))
  (bind _ownerenemy_2 (`self.OwnerEnemy`))
  (if (`/Game/Blueprint/BP_ZZZ_EnemyBase.CheckPlayerInNormalAttackRange` (`self.OwnerEnemy`))
    ; Comment
    (`/Game/Blueprint/Interface/BPI_IEnemyStateMachine.ChangeState` (`/Game/Blueprint/Claymore/State/BP_Claymore.AC_ClaymoreStateMachine` _ownerenemy_2) (`/Game/Blueprint/Claymore/State/BP_Claymore.AC_ClaymoreIdleState` _ownerenemy_2))
    (else
      ; Comment
      (`/Game/Blueprint/BP_ZZZ_EnemyBase.Turn` _ownerenemy)
      (`/Game/Blueprint/BP_ZZZ_EnemyBase.Walk` _ownerenemy))))

(event `self.Exit`
  ; Comment
  (set `/Game/Blueprint/Claymore/State/BP_Claymore.isWalking?` false (`self.OwnerEnemy`)))