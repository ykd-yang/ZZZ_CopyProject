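; Hit-reaction state component for the Claymore enemy, used by its enemy state machine.
; On BeginPlay it casts its owner to BP_Claymore and stores it as EnemyOwner.
; Entering the state clears any pending knockback timer, plays the hit montage and starts a new short timer.
; When that timer expires, the state machine switches to idle, independent of montage completion.
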(event `self.ReceiveBeginPlay`
  ; 변수 설정
  (bind _asbp_claymore (cast `/Game/Blueprint/Claymore/State/BP_Claymore` (`self.GetOwner`)))
  (set `self.EnemyOwner` _asbp_claymore))

(event `/Game/Blueprint/Interface/BPI_IEnemyState.Enter`
  (`KismetSystemLibrary.K2_ClearAndInvalidateTimerHandle` (`self.KnockBackTimer`))
  ; 적중 애니메이션 재생
  (`|PlayMontage` (`Character.Mesh` (`self.EnemyOwner`)) "/Game/Enemy/ModifiedClaymore/Animation/Montage/AM_EnemyHit.AM_EnemyHit"
    (:`then`
      ; 넉백 탈출을 위한 타이머
      (bind _returnvalue (`KismetSystemLibrary.K2_SetTimerDelegate` (delegate `KnockBackExpired`) 1.5))
      (set `self.KnockBackTimer` _returnvalue))))

(event `KnockBackExpired`
  (bind _enemyowner (`self.EnemyOwner`))
  ; 넉백 탈출을 위한 타이머
  (`/Game/Blueprint/Claymore/State/AC_ClaymoreStateMachine.ChangeState` (`/Game/Blueprint/Claymore/State/BP_Claymore.AC_EnemyStateMachine` _enemyowner) (`/Game/Blueprint/Claymore/State/BP_Claymore.AC_EnemyIdleState` _enemyowner)))