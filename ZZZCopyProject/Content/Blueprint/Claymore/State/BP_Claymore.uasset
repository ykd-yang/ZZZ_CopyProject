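; BP_Claymore is an enemy whose state machine starts in Idle, runs on Tick after spawning, and switches to Hit or Dead on damage events.
; Hits apply knockback, show damage numbers and spawn Niagara VFX, which attack warnings reuse.
; Helper functions move it toward the player without sweep and yaw it to face them.
; Turn targeting uses a range-box overlap plus an FOV test that compares the actor's location with itself.
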(event `self.ReceiveBeginPlay`
  (`parent.ReceiveBeginPlay`)
  (`/Game/Blueprint/Interface/BPI_IEnemyStateMachine.ChangeState` (`self.AC_EnemyStateMachine`) (`self.AC_EnemyIdleState`))
  (set `self.HP` 1000))

(event `self.ReceiveTick`
  (params (DeltaSeconds :type "Float (single-precision)"))
  (if (`self.EndSpawn`)
    (`/Game/Blueprint/Interface/BPI_IEnemyStateMachine.Execute` (`self.AC_EnemyStateMachine`))))

(event `/Game/Blueprint/Interface/Behivour/BPI_Common_Behaviour.Dead`
  (params (KnockBack :type "Vector Structure"))
  ; Comment
  (`/Game/Blueprint/Interface/BPI_IEnemyStateMachine.ChangeState` (`self.AC_EnemyStateMachine`) (`self.AC_EnemyDeadState`))
  (`self.KnockBack` KnockBack))

(event `/Game/Blueprint/Interface/Behivour/BPI_Common_Behaviour.Damaged`
  (params (KnockBack :type "Vector Structure") (Damage :type Integer))
  ; 적중 시 상태 전환
  (`/Game/Blueprint/Interface/BPI_IEnemyStateMachine.ChangeState` (`self.AC_EnemyStateMachine`) (`self.AC_EnemyHitState`))
  (`self.KnockBack` KnockBack)
  (bind _aswb_damage_display (cast `/Game/Blueprint/UI/Damage/WB_DamageDisplay` (`WidgetComponent.GetUserWidgetObject` (`self.Widget`))))
  (`/Game/Blueprint/UI/Damage/WB_DamageDisplay.DisplayDamage` _aswb_damage_display (`KismetMathLibrary.Conv_IntToInt64` Damage))
  (`self.PlayVFX`))

(event `/Game/Blueprint/Interface/BPI_ShowVFX.PlayAttackWarning`
  ; 경고 출력 인터페이스
  (`self.PlayVFX`))

(event `Key|K`
  (params (Key :type "Key Structure")))

(fn `AttackTargeting`
  (bind _infov (`self.CheckFov`))
  (if _infov
    (`self.Turn`)))

(fn `CheckFov`
  (returns (InFov :type Boolean))
  (bind _in_attack_range_ (`self.CheckPlayerInAttackRange`))
  (return (and _in_attack_range_ (<= (`KismetMathLibrary.RadiansToDegrees` (`KismetMathLibrary.Dot_VectorVector` (`KismetMathLibrary.Normal` (- (`self.K2_GetActorLocation`) (`self.K2_GetActorLocation` self))) (`KismetMathLibrary.Normal` (`self.GetActorForwardVector` self)))) (`self.FovAngle`)))))

(fn `CheckPlayerInAttackRange`
  (returns (`In Attack Range?` :type Boolean))
  (return (`KismetArrayLibrary.Array_IsNotEmpty` (`PrimitiveComponent.GetOverlappingActors` (`self.AttackRangeBox`) "/Game/Blueprint/BP_ZZZ_AgentBase.BP_ZZZ_AgentBase_C"))))

(fn `PlayVFX`
  (bind _mesh (`self.Mesh`))
  (bind _returnvalue (`NiagaraFunctionLibrary.SpawnSystemAttached` "/Game/SlashHitVFX/NS/NS_Hit_Sword.NS_Hit_Sword" _mesh "None" (.location (`SkinnedAsset.FindSocketInfo` (`SkinnedMeshComponent.SkinnedAsset` _mesh) "headParticleSocket")) (struct) "KeepWorldPosition" true))
  (`SceneComponent.SetWorldScale3D` _returnvalue (5.0 5.0 5.0)))

(fn `Turn`
  (bind (_returnvalue_x _returnvalue_y) (`KismetMathLibrary.BreakVector` (- (`self.K2_GetActorLocation` (`self.Player`)) (`self.K2_GetActorLocation`))))
  (`self.K2_SetActorRotation` (`KismetMathLibrary.MakeRotator` 0.0 0.0 (`KismetMathLibrary.RadiansToDegrees` (`KismetMathLibrary.Atan2` _returnvalue_y _returnvalue_x))))
  (return))

(fn `UserConstructionScript`)

(fn `Walking`
  (locals (Dir :type "Vector Structure" :default (0.0 0.0 0.0)))
  (bind _output_get (set `local.Dir` (`KismetMathLibrary.Normal` (- (`self.K2_GetActorLocation` (`self.Player`)) (`self.K2_GetActorLocation`)))))
  (`self.K2_SetActorLocation` (+ (* (* (`self.Speed`) (`GameplayStatics.GetWorldDeltaSeconds`)) _output_get) (`self.K2_GetActorLocation`))))