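; Game mode for a boss stage that opens with a dialogue and manages music, player input and the mouse cursor around it.
; BeginPlay starts the dialogue widget and stage-parameterized audio cue; dialogue and selection events rebroadcast through dispatchers.
; Dialogue end plays a fade sequence, blends to another camera, switches music, restores input and later adds the agent HP bar.
; DieBoss binds the dialogue-end dispatcher to open the stage-select level after a delay.
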(event `self.ReceiveBeginPlay`
  (bind _soundcue (`self.SoundCue`))
  (bind _returnvalue (`AddComponent|NODE_AddAudioComponent-7`))
  (set `self.SoundCue` _returnvalue)
  (set `self.PlayerCharacter` (`GameplayStatics.GetPlayerCharacter` 0))
  ; 다이얼로그 위젯 뷰포트에 추가
  (bind _returnvalue_2 (`|CreateWidget` "/Game/Blueprint/UI/Dialogue/WBP_DialogueSystem.WBP_DialogueSystem_C" (`GameplayStatics.GetPlayerController` 0)))
  (bind _output_get (set `self.Dialogue` _returnvalue_2))
  (`UserWidget.AddToViewport` _output_get 0)
  (`/Game/Blueprint/UI/Dialogue/WBP_DialogueSystem.StartDialogue` _output_get "/Game/Blueprint/UI/Dialogue/DT_Dialogue.DT_Dialogue")
  (`AudioComponent.SetIntParameter` _soundcue "CurrentStage" 0)
  (`AudioComponent.Play` _soundcue 0.0))

(event `OnDialogueBegin`
  ; Comment
  (`self.DisableInput` (`self.PlayerCharacter`) (`GameplayStatics.GetPlayerController` 0))
  (`self.OnDialogueBegin_Dispatcher`))

(event `OnDialogueEnd`
  (bind _returnvalue (`GameplayStatics.GetPlayerController` 0))
  (bind _soundcue (`self.SoundCue`))
  ; Comment
  ;; 대화가 끝나면 페이드인 시퀀스 재생
  (bind _outactor (`LevelSequencePlayer.CreateLevelSequencePlayer` "/Game/Sequence/FadeIn.FadeIn"))
  (`MovieSceneSequencePlayer.Play` (`LevelSequenceActor.SequencePlayer` _outactor))
  (`AudioComponent.FadeOut` (`self.SoundCue`) 2.0 0.0 "Linear")
  (`KismetSystemLibrary.Delay` 1.8)
  ; 페이드인 끝나고 검은색 큐브로의 시점 전환 후 디스패처를 이용한 효과
  (`PlayerController.SetViewTargetWithBlend` _returnvalue (`self.CameraActor2`) 0.0 "VTBlend_Linear" 0.0 false)
  (`AudioComponent.SetIntParameter` _soundcue "CurrentStage" 1)
  (`AudioComponent.FadeIn` _soundcue 2.0 1.0 0.0 "Linear")
  (bind _asbp_camera_actor (cast `/Game/Blueprint/BP_CameraActor` (`self.CameraActor2`)))
  ; 캐릭터 인풋 정상화
  (`/Game/Blueprint/BP_CameraActor.ChangedView` _asbp_camera_actor)
  (`self.EnableInput` (`self.PlayerCharacter`) _returnvalue)
  (`self.OnDialogueEnd_Dispatcher`)
  (`AudioComponent.SetIntParameter` (`self.SoundCue`) "CurrentStage" 1)
  (`KismetSystemLibrary.Delay` 4.0)
  (bind _returnvalue_2 (`|CreateWidget` "/Game/Blueprint/UI/HpBar/WBP_AgentHpBar.WBP_AgentHpBar_C" (`GameplayStatics.GetPlayerController` 0)))
  (`UserWidget.AddToViewport` _returnvalue_2 0))

(event `OnSelectionBegin`
  ; Comment
  (set `PlayerController.bShowMouseCursor` true (`GameplayStatics.GetPlayerController` 0))
  (`self.OnSelectionBegin_Dispatcher`))

(event `OnSelectionEnd`
  ; Comment
  (set `PlayerController.bShowMouseCursor` false (`GameplayStatics.GetPlayerController` 0))
  (`self.OnSelectionEnd_Dispatcher`))

(event `DieBoss`
  (add `self.OnDialogueEnd_Dispatcher` (delegate `CustomEvent`))
  (`KismetSystemLibrary.PrintString` "Hello"))

(event `CustomEvent`
  (`KismetSystemLibrary.Delay` 3.0)
  (`KismetSystemLibrary.PrintString` "Open LEvel!")
  (`GameplayStatics.OpenLevelBySoftObjectPtr` "/Game/Maps/AlphaDemo/AlphaStageSelect.AlphaStageSelect"))

(fn `UserConstructionScript`)