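; Game mode Blueprint, by its name, that runs a dialogue sequence as soon as play begins.
; BeginPlay caches the player character, adds a WBP_DialogueSystem widget to the viewport and starts it with the DT_Dialogue table.
; Dialogue begin and end events disable and restore player input, while selection begin and end events toggle the mouse cursor.
; Each of these events also calls a matching dispatcher to notify listeners.
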(event `self.ReceiveBeginPlay`
  (set `self.PlayerCharacter` (`GameplayStatics.GetPlayerCharacter` 0))
  ; 다이얼로그 위젯 뷰포트에 추가
  (bind _returnvalue (`|CreateWidget` "/Game/Blueprint/UI/Dialogue/WBP_DialogueSystem.WBP_DialogueSystem_C" (`GameplayStatics.GetPlayerController` 0)))
  (bind _output_get (set `self.Dialogue` _returnvalue))
  (`UserWidget.AddToViewport` _output_get 0)
  (`/Game/Blueprint/UI/Dialogue/WBP_DialogueSystem.StartDialogue` _output_get "/Game/Blueprint/UI/Dialogue/DT_Dialogue.DT_Dialogue"))

(event `OnDialogueBegin`
  ; Comment
  (`self.DisableInput` (`self.PlayerCharacter`) (`GameplayStatics.GetPlayerController` 0))
  (`self.OnDialogueBegin_Dispatcher`))

(event `OnDialogueEnd`
  ; Comment
  (`self.EnableInput` (`self.PlayerCharacter`) (`GameplayStatics.GetPlayerController` 0))
  (`self.OnDialogueEnd_Dispatcher`))

(event `OnSelectionBegin`
  ; Comment
  (set `PlayerController.bShowMouseCursor` true (`GameplayStatics.GetPlayerController` 0))
  (`self.OnSelectionBegin_Dispatcher`))

(event `OnSelectionEnd`
  ; Comment
  (set `PlayerController.bShowMouseCursor` false (`GameplayStatics.GetPlayerController` 0))
  (`self.OnSelectionEnd_Dispatcher`))

(fn `UserConstructionScript`)