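; AC_DurahanIdleState is the idle state component for the Durahan boss, used by its state machine.
; BeginPlay caches the owning BP_Boss, and Enter clears the boss's IsWalking flag.
; Update rolls a random percentage and asks ACDurahanStateMachine to change state, but both branches currently select the attack state, so the roll has no effect on the outcome.
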(event `self.ReceiveBeginPlay`
  ; Comment
  (bind _asbp_boss (cast `/Game/Blueprint/Boss/BP_Boss` (`self.GetOwner`)))
  (set `self.OwnerEnemy` _asbp_boss))

(event `/Game/Blueprint/Interface/BPI_IEnemyState.Update`
  (bind _ownerenemy (`self.OwnerEnemy`))
  (bind _ownerenemy_2 (`self.OwnerEnemy`))
  (if (>= (`KismetMathLibrary.RandomIntegerInRange` 1 100) 40)
    ; Comment
    (`/Game/Blueprint/Interface/BPI_IEnemyStateMachine.ChangeState` (`/Game/Blueprint/Boss/BP_Boss.AC_DurahanStateMachine` _ownerenemy) (`/Game/Blueprint/Boss/BP_Boss.AC_DurahanAttackState` _ownerenemy))
    (else
      ; Comment
      (`/Game/Blueprint/Interface/BPI_IEnemyStateMachine.ChangeState` (`/Game/Blueprint/Boss/BP_Boss.AC_DurahanStateMachine` _ownerenemy_2) (`/Game/Blueprint/Boss/BP_Boss.AC_DurahanAttackState` _ownerenemy_2)))))

(event `/Game/Blueprint/Interface/BPI_IEnemyState.Enter`
  (set `/Game/Blueprint/Boss/BP_Boss.IsWalking` false (`self.OwnerEnemy`)))