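; Boss walk state component for the boss's state machine, driving movement relative to the player.
; Each Update checks player distance, switching to Idle within attack range or randomly choosing Charge Attack or walking within dash range.
; Outside both ranges the boss turns, then walks.
; Enter and Exit both set IsWalking to true, and Exit also prints a debug message.
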(event `/Game/Blueprint/Boss/BPI_IState.Update`
  (params (Boss :type "/Game/Blueprint/Boss/BP_Boss Object Reference"))
  (bind _boss (`self.Boss`))
  (bind _boss_2 (`self.Boss`))
  (bind (_canattackdistance _candashattackdistance) (`/Game/Blueprint/Boss/BP_Boss.CheckDistanceWithPlayer` Boss))
  (if _canattackdistance
    (message `/Game/Blueprint/Boss/BPI_IStateMachine.ChangeState` (`/Game/Blueprint/Boss/BP_Boss.AC_StateMachine` _boss) (`/Game/Blueprint/Boss/BP_Boss.AC_IdleState` _boss) _boss)
    (elif _candashattackdistance
      (if (>= (`KismetMathLibrary.RandomIntegerInRange` 0 100) 60)
        (message `/Game/Blueprint/Boss/BPI_IStateMachine.ChangeState` (`/Game/Blueprint/Boss/BP_Boss.AC_StateMachine` _boss_2) (`/Game/Blueprint/Boss/BP_Boss.AC_ChargeAttackState` _boss_2) _boss_2)
        (else
          (`/Game/Blueprint/Boss/BP_Boss.Walking` _boss :!label _label)))
      (else
        (`/Game/Blueprint/Boss/BP_Boss.Turn` _boss _boss)
        (goto _label)))))

(event `/Game/Blueprint/Boss/BPI_IState.Exit`
  (params (Boss :type "/Game/Blueprint/Boss/BP_Boss Object Reference"))
  (`KismetSystemLibrary.PrintString` "워크상태 나감")
  (set `/Game/Blueprint/Boss/BP_Boss.IsWalking` true Boss))

(event `/Game/Blueprint/Boss/BPI_IState.Enter`
  (params (Boss :type "/Game/Blueprint/Boss/BP_Boss Object Reference"))
  (bind _output_get (set `self.Boss` Boss))
  (set `/Game/Blueprint/Boss/BP_Boss.IsWalking` true _output_get))