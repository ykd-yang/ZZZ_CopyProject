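; Boss state machine component that holds the current state and switches between interface-based state objects.
; Execute runs Update on the current state, or assigns the boss's idle state without calling Enter when none is valid.
; ChangeState calls Exit on the state read from the boss and Enter on the new one, then records it in the component's own CurrentState.
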(event `self.ReceiveBeginPlay`)

(event `/Game/Blueprint/Boss/BPI_IStateMachine.Execute`
  (params (Boss :type "/Game/Blueprint/Boss/BP_Boss Object Reference"))
  (bind _currentstate (`self.CurrentState`))
  (if (`KismetSystemLibrary.IsValidInterface` _currentstate)
    (`/Game/Blueprint/Boss/BPI_IState.Update` _currentstate Boss)
    (else
      (set `self.CurrentState` (`/Game/Blueprint/Boss/BP_Boss.AC_IdleState` Boss)))))

(fn `ChangeState`
  (params (ChangeState :type "/Game/Blueprint/Boss/AC_StateBase Object Reference") (Boss :type "/Game/Blueprint/Boss/BP_Boss Object Reference"))
  (locals (BossObject :type "/Game/Blueprint/Boss/BP_Boss Object Reference") (ChageState :type "/Game/Blueprint/Boss/BPI_IState Interface") (NewLocalVar :type "/Game/Blueprint/Boss/BP_Boss Object Reference"))
  (bind _currentstate (`/Game/Blueprint/Boss/BP_Boss.CurrentState` Boss))
  (bind _chagestate (`local.ChageState`))
  (bind _chagestate_2 (`local.ChageState`))
  (set `local.ChageState` ChangeState)
  (set `local.BossObject` Boss)
  (if (`KismetSystemLibrary.IsValidInterface` _currentstate)
    (bind _output_get (set `self.PrevieousState` _currentstate))
    (`/Game/Blueprint/Boss/BPI_IState.Exit` _output_get (`local.BossObject`))
    (if (`KismetSystemLibrary.IsValidInterface` _chagestate)
      (`/Game/Blueprint/Boss/BPI_IState.Enter` _chagestate (`local.BossObject`))
      (set `self.CurrentState` _chagestate)
      (else
        (bind _output_get_2 (set `self.CurrentState` _chagestate_2 :!label _label))
        (set `self.PrevieousState` _output_get_2)))
    (else
      (`/Game/Blueprint/Boss/BPI_IState.Enter` _chagestate_2 (`local.BossObject`))
      (goto _label)))
  (return))