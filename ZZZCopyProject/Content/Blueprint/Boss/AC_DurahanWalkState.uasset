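; Walk state component for the Durahan boss's state machine, handling its movement toward attacks on the player.
; It caches the owning BP_Boss on BeginPlay and toggles its IsWalking flag on Enter and Exit.
; Each Update switches to Idle when the player is in normal attack range, requests the charge attack within a fixed distance, and otherwise turns and walks.
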(event `self.ReceiveBeginPlay`
  ; Comment
  (bind _asbp_boss (cast `/Game/Blueprint/Boss/BP_Boss` (`self.GetOwner`)))
  (set `self.OwnerEnemy` _asbp_boss))

(event `/Game/Blueprint/Interface/BPI_IEnemyState.Update`
  (bind _ownerenemy (`self.OwnerEnemy`))
  (bind _ownerenemy_2 (`self.OwnerEnemy`))
  (bind _ownerenemy_3 (`self.OwnerEnemy`))
  (if (`/Game/Blueprint/BP_ZZZ_EnemyBase.CheckPlayerInNormalAttackRange` (`self.OwnerEnemy`))
    ; Comment
    (`/Game/Blueprint/Interface/BPI_IEnemyStateMachine.ChangeState` (`/Game/Blueprint/Boss/BP_Boss.AC_DurahanStateMachine` _ownerenemy_2) (`/Game/Blueprint/Boss/BP_Boss.AC_DurahanIdleState` _ownerenemy_2))
    (elif (<= (`KismetMathLibrary.Vector_Distance` (`Actor.K2_GetActorLocation` _ownerenemy) (`Actor.K2_GetActorLocation` (`/Game/Blueprint/BP_ZZZ_EnemyBase.Player` _ownerenemy))) 700.0)
      ; Comment
      (message `/Game/Blueprint/Interface/BPI_IEnemyStateMachine.ChangeState` (`/Game/Blueprint/Boss/BP_Boss.AC_DurahanStateMachine` _ownerenemy_3) (`/Game/Blueprint/Boss/BP_Boss.AC_DurahanChargeAttackState` _ownerenemy_3))
      (else
        ; Comment
        (`/Game/Blueprint/BP_ZZZ_EnemyBase.Turn` (`self.OwnerEnemy`))
        (`/Game/Blueprint/BP_ZZZ_EnemyBase.Walk` (`self.OwnerEnemy`))))))

(event `/Game/Blueprint/Interface/BPI_IEnemyState.Enter`
  (set `/Game/Blueprint/Boss/BP_Boss.IsWalking` true (`self.OwnerEnemy`)))

(event `/Game/Blueprint/Interface/BPI_IEnemyState.Exit`
  (set `/Game/Blueprint/Boss/BP_Boss.IsWalking` false (`self.OwnerEnemy`)))