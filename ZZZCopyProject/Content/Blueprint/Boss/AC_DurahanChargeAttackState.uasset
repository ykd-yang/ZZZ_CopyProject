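; Actor component state for the Durahan boss that performs its charge (dash) attack.
; On BeginPlay it caches the owning BP_Boss; on Enter it turns the boss and plays the AM_Dash montage.
; Montage completion switches the Durahan state machine to the waiting state.
; Interruption only prints the first actor overlapping the boss's capsule, without changing state.
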(event `self.ReceiveBeginPlay`
  ; Comment
  (bind _asbp_boss (cast `/Game/Blueprint/Boss/BP_Boss` (`self.GetOwner`)))
  (set `self.OwnerEnemy` _asbp_boss))

(event `/Game/Blueprint/Interface/BPI_IEnemyState.Enter`
  (bind _ownerenemy (`self.OwnerEnemy`))
  (bind _ownerenemy_2 (`self.OwnerEnemy`))
  ; Comment
  (`/Game/Blueprint/BP_ZZZ_EnemyBase.Turn` _ownerenemy_2)
  (`|PlayMontage` (`Character.Mesh` _ownerenemy_2) "/Game/Enemy/ModifiedDurahan/Animation/AM_Dash.AM_Dash"
    (:`OnCompleted`
      (`/Game/Blueprint/Interface/BPI_IEnemyStateMachine.ChangeState` (`/Game/Blueprint/Boss/BP_Boss.AC_DurahanStateMachine` _ownerenemy) (`/Game/Blueprint/Boss/BP_Boss.AC_DurahanWaitingState` _ownerenemy)))
    (:`OnInterrupted`
      (`KismetSystemLibrary.PrintString` (`KismetSystemLibrary.GetDisplayName` (`|GetArrayItem` (`PrimitiveComponent.GetOverlappingActors` (`Character.CapsuleComponent` _ownerenemy) null)))))))