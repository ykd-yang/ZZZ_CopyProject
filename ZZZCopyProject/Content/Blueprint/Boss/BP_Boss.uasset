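; Boss enemy that hunts the player pawn, with its behavior driven by a component-style state machine ticked once spawning ends.
; It supplies helpers for states: attack and dash range checks, FOV-gated targeting, yaw turning and direct location-based movement without sweep.
; A timeline scales the attack warning cone in and out.
; Damage routes to the character base's hit event; death has a state change and a montage event that destroys the actor.
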(event `BossWarning`
  (bind (_direction _newtrack_0) (`Timeline|Timeline` :!label _label)
    (:`Update`
      (`SceneComponent.SetWorldScale3D` (`self.Warningcone`) (`KismetMathLibrary.MakeVector` _newtrack_0 _newtrack_0 0.01)))))

(event `BossWarningEnd`
  (goto _label :!via `Reverse`))

(event `/Game/Blueprint/Interface/BPI_Behaivour.GetHit`)

(event `self.ReceiveBeginPlay`
  (bind _ac_idlestate (`self.AC_IdleState`))
  ; 스테이트 초기화 및 플레이어 변수 초기화
  (`/Game/Blueprint/Boss/BPI_IStateMachine.ChangeState` (`self.AC_StateMachine`) _ac_idlestate self)
  (bind _output_get (set `self.Player` (`GameplayStatics.GetPlayerPawn` 0)))
  (set `self.CurrentState` _ac_idlestate)
  (if (`KismetSystemLibrary.IsValid` _output_get)
    (set `self.Speed` 600.0)))

(event `self.ReceiveTick`
  (params (DeltaSeconds :type "Float (single-precision)"))
  (if (`self.EndSpawn`)
    (`/Game/Blueprint/Boss/BPI_IStateMachine.Execute` (`self.AC_StateMachine`) self)))

(event `/Game/Blueprint/Interface/BPI_Behaivour.PlayDeath`
  (`|PlayMontage` (`self.Mesh`) "/Game/Enemy/ModifiedDurahan/Animation/AM_BossDie.AM_BossDie"
    (:`then`
      (`KismetSystemLibrary.Delay` 3.0)
      (`self.K2_DestroyActor`))))

(fn `AttackTargeting`
  (bind _infov (`self.CheckInFov` self))
  (if _infov
    (`self.Turn` self self)))

(fn `CheckDistanceWithPlayer`
  (returns (CanAttackDistance :type Boolean) (CanDashAttackDistance :type Boolean))
  (bind _returnvalue (<= (`KismetMathLibrary.Vector_Distance` (`self.K2_GetActorLocation` (`self.Player`)) (`self.K2_GetActorLocation` self)) (`self.DashRange`)))
  (if (`KismetArrayLibrary.Array_IsEmpty` (`PrimitiveComponent.GetOverlappingActors` (`self.NomalAttackDetectCollider`) "/Game/Blueprint/BP_ZZZ_AgentBase.BP_ZZZ_AgentBase_C"))
    (return false _returnvalue)
    (else
      (return true _returnvalue))))

(fn `CheckInFov`
  (returns (InFov :type Boolean))
  (bind _canattackdistance (`self.CheckDistanceWithPlayer`))
  (return (and (<= (`KismetMathLibrary.RadiansToDegrees` (`KismetMathLibrary.Dot_VectorVector` (`KismetMathLibrary.Normal` (- (`self.K2_GetActorLocation` (`self.Player`)) (`self.K2_GetActorLocation` self))) (`KismetMathLibrary.Normal` (`self.GetActorForwardVector` self)))) (`self.FovAngle`)) _canattackdistance)))

(fn `Die`
  (`/Game/Blueprint/Boss/AC_StateMachine.ChangeState` (`self.AC_StateMachine`) (`self.AC_DeadState`) self))

(fn `TakeDamage`
  (bind _player (`self.Player`))
  (bind _asbp_zzz_character_base (cast `/Game/Blueprint/BP_ZZZ_CharacterBase` self))
  ; 01. 죽었는지 검사
  (if (not (`/Game/Blueprint/BP_ZZZ_CharacterBase.IsDead?` _asbp_zzz_character_base))
    (bind _asbp_zzz_character_base_2 (cast `/Game/Blueprint/BP_ZZZ_CharacterBase` self))
    (`self.OnCharacterHItEvent` _asbp_zzz_character_base_2 _player)
    (bind _asbp_zzz_agent_base (cast `/Game/Blueprint/BP_ZZZ_AgentBase` _player))
    (if (`/Game/Blueprint/BP_ZZZ_CharacterBase.IsDead?` _asbp_zzz_character_base_2)
      _)))

(fn `Turn`
  (params (BossVariable :type "/Game/Blueprint/Boss/BP_Boss Object Reference"))
  (bind (_returnvalue_x _returnvalue_y) (`KismetMathLibrary.BreakVector` (- (`self.K2_GetActorLocation` (`self.Player`)) (`self.K2_GetActorLocation` BossVariable))))
  (`self.K2_SetActorRotation` BossVariable (`KismetMathLibrary.MakeRotator` 0.0 0.0 (`KismetMathLibrary.RadiansToDegrees` (`KismetMathLibrary.Atan2` _returnvalue_y _returnvalue_x))) false)
  (return))

(fn `UserConstructionScript`)

(fn `Walking`
  (locals (Dir :type "Vector Structure"))
  (bind _output_get (set `local.Dir` (`KismetMathLibrary.Normal` (- (`self.K2_GetActorLocation` (`self.Player`)) (`self.K2_GetActorLocation`)))))
  (`self.K2_SetActorLocation` (+ (* (* (`self.Speed`) (`GameplayStatics.GetWorldDeltaSeconds`)) _output_get) (`self.K2_GetActorLocation`))))