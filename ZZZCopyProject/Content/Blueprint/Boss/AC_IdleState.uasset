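; Boss idle state component that picks the boss's next state from its distance to the player.
; While the boss is alive, Update switches to the attack state in attack range and otherwise to walk.
; Within dash-attack range, a random roll can instead trigger a ChangeState call, though that call has no target state set.
; Enter and Exit only print debug messages.
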(event `/Game/Blueprint/Boss/BPI_IState.Exit`
  (params (Boss :type "/Game/Blueprint/Boss/BP_Boss Object Reference"))
  (`KismetSystemLibrary.PrintString` "아이들 상태 나감"))

(event `/Game/Blueprint/Boss/BPI_IState.Update`
  (params (Boss :type "/Game/Blueprint/Boss/BP_Boss Object Reference"))
  (bind _ac_statemachine (`/Game/Blueprint/Boss/BP_Boss.AC_StateMachine` Boss))
  (if (not (`/Game/Blueprint/BP_ZZZ_CharacterBase.IsDead?` Boss))
    ; 거리 판단(공격범위가 아니라면 Walk State로 전환)
    (bind (_canattackdistance _candashattackdistance) (`/Game/Blueprint/Boss/BP_Boss.CheckDistanceWithPlayer` Boss))
    ; 상태전환
    (if _canattackdistance
      (message `/Game/Blueprint/Boss/BPI_IStateMachine.ChangeState` _ac_statemachine (`/Game/Blueprint/Boss/BP_Boss.AC_AttackState` Boss) Boss)
      (elif (and _candashattackdistance (>= (`KismetMathLibrary.RandomIntegerInRange` 1 100) 60))
        (`/Game/Blueprint/Boss/AC_StateMachine.ChangeState` _ac_statemachine null Boss)
        (else
          (`/Game/Blueprint/Boss/AC_StateMachine.ChangeState` _ac_statemachine (`/Game/Blueprint/Boss/BP_Boss.AC_WalkState` Boss) Boss))))))

(event `/Game/Blueprint/Boss/BPI_IState.Enter`
  (params (Boss :type "/Game/Blueprint/Boss/BP_Boss Object Reference"))
  (`KismetSystemLibrary.PrintString` "아이들 상태 진입"))