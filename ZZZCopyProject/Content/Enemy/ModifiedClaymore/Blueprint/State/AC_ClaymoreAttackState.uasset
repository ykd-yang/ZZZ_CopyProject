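; Attack state component for the Claymore enemy, used by its state machine component.
; On BeginPlay it caches the owning BP_Claymore.
; On Enter it turns the enemy, plays the attack montage, and switches the state machine back to idle when the montage completes.
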(event `self.ReceiveBeginPlay`
  ; 초기화
  (bind _asbp_claymore (cast `/Game/Enemy/ModifiedClaymore/Blueprint/State/BP_Claymore` (`self.GetOwner`)))
  (set `self.OwnerEnemy` _asbp_claymore))

(event `self.Enter`
  (bind _ownerenemy (`self.OwnerEnemy`))
  (bind _ownerenemy_2 (`self.OwnerEnemy`))
  (`/Game/Blueprint/BP_ZZZ_EnemyBase.Turn` _ownerenemy_2)
  (`|PlayMontage` (`Character.Mesh` _ownerenemy_2) "/Game/Enemy/ModifiedClaymore/Animation/Montage/AM_EnemyAttack.AM_EnemyAttack"
    (:`OnCompleted`
      (`/Game/Blueprint/Interface/BPI_IEnemyStateMachine.ChangeState` (`/Game/Enemy/ModifiedClaymore/Blueprint/State/BP_Claymore.AC_ClaymoreStateMachine` _ownerenemy) (`/Game/Enemy/ModifiedClaymore/Blueprint/State/BP_Claymore.AC_ClaymoreIdleState` _ownerenemy)))))