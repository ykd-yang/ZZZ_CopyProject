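; BP_Claymore is the Claymore enemy, driven by a state machine component that starts in Idle and executes every tick.
; Damage and death events switch it to Hit or Dead and apply knockback; hits also display damage on a widget and spawn a Niagara effect, while death fires a signal.
; Helper functions report agent overlap in the normal attack range box and expose the attack detection box and mesh.
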(event `self.ReceiveBeginPlay`
  ; 초기화
  (`parent.ReceiveBeginPlay`)
  (`/Game/Blueprint/Interface/BPI_IEnemyStateMachine.ChangeState` (`self.AC_ClaymoreStateMachine`) (`self.AC_ClaymoreIdleState`))
  (set `self.HP` 1000))

(event `self.ReceiveTick`
  (params (DeltaSeconds :type "Float (single-precision)"))
  ; 상태 머신 실행
  (`/Game/Blueprint/Interface/BPI_IEnemyStateMachine.Execute` (`self.AC_ClaymoreStateMachine`)))

(event `/Game/Blueprint/Interface/Behivour/BPI_Common_Behaviour.Dead`
  (params (KnockBack :type "Vector Structure"))
  ; 사망 시 상태 전환
  (`self.DeadSignal`)
  (`/Game/Blueprint/Interface/BPI_IEnemyStateMachine.ChangeState` (`self.AC_ClaymoreStateMachine`) (`self.AC_ClaymoreDeadState`))
  (`self.KnockBack` KnockBack))

(event `/Game/Blueprint/Interface/Behivour/BPI_Common_Behaviour.Damaged`
  (params (KnockBack :type "Vector Structure") (Damage :type Integer) (HitParticle :type "NiagaraComponent Object Reference") (HitParticleScale :type "Float (double-precision)"))
  ; 적중 시 상태 전환
  (`/Game/Blueprint/Interface/BPI_IEnemyStateMachine.ChangeState` (`self.AC_ClaymoreStateMachine`) (`self.AC_ClaymoreHitState`))
  (`self.KnockBack` KnockBack)
  (bind _aswb_damage_display (cast `/Game/Blueprint/UI/Damage/WB_DamageDisplay` (`WidgetComponent.GetUserWidgetObject` (`self.Widget`))))
  (`/Game/Blueprint/UI/Damage/WB_DamageDisplay.DisplayDamage` _aswb_damage_display (`KismetMathLibrary.Conv_IntToInt64` Damage))
  (`self.PlayHitEffect` "/Game/VFX/SlashHitVFX/NS/NS_Hit_Sword.NS_Hit_Sword" 5.0))

(fn `CheckPlayerInNormalAttackRange`
  (returns (`Player In Attack Range` :type Boolean))
  (return (`KismetArrayLibrary.Array_IsNotEmpty` (`PrimitiveComponent.GetOverlappingActors` (`self.NormalAttackRangeBox`) "/Game/Blueprint/BP_ZZZ_AgentBase.BP_ZZZ_AgentBase_C"))))

(fn `GetAttackDetectBox`
  (returns (Box :type "BoxComponent Object Reference"))
  (return (`self.AttackDetectBox`)))

(fn `GetMesh`
  (returns (`Mesh Comp` :type "MeshComponent Object Reference"))
  (return (`self.Mesh`)))

(fn `UserConstructionScript`)