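; BP_Boss is the Durahan boss enemy, whose death opens the AlphaStageSelect level after a delay.
; A state machine component starts in Idle, runs on Tick once spawning ends, and changes state on damage or death.
; Hits add knockback, a damage-number widget and Niagara effects.
; A timeline scales a reversible warning cone, while helper functions expose mesh, attack box and player-in-range checks; dialogue and game-mode boss-kill logic is unwired.
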(event `BossWarning`
  (bind _warningcone (`self.Warningcone`))
  (bind (_direction _newtrack_0) (`Timeline|Timeline` :!label _label)
    (:`Update`
      (`SceneComponent.SetWorldScale3D` _warningcone (`KismetMathLibrary.MakeVector` _newtrack_0 _newtrack_0 0.01)))
    (:`Finished`
      (`SceneComponent.SetWorldScale3D` _warningcone (`KismetMathLibrary.MakeVector` _newtrack_0 _newtrack_0 0.01)))))

(event `BossWarningEnd`
  (goto _label :!via `Reverse`))

(event `self.ReceiveBeginPlay`
  ; 초기화
  (`parent.ReceiveBeginPlay`)
  (`/Game/Blueprint/Interface/BPI_IEnemyStateMachine.ChangeState` (`self.AC_DurahanStateMachine`) (`self.AC_DurahanIdleState`))
  (set `self.HP` 1000))

(event `self.ReceiveTick`
  (params (DeltaSeconds :type "Float (single-precision)"))
  ; 상태 머신 실행
  (if (`self.EndSpawn`)
    (`/Game/Blueprint/Interface/BPI_IEnemyStateMachine.Execute` (`self.AC_DurahanStateMachine`))))

(event `/Game/Blueprint/Interface/Behivour/BPI_Common_Behaviour.Dead`
  (params (KnockBack :type "Vector Structure"))
  ; 사망 시
  (`self.DeadSignal`)
  (`/Game/Blueprint/Interface/BPI_IEnemyStateMachine.ChangeState` (`self.AC_DurahanStateMachine`) (`self.AC_DurahanDeadState`))
  (`self.KnockBack` KnockBack)
  (`KismetSystemLibrary.Delay` 5.0)
  (`GameplayStatics.OpenLevelBySoftObjectPtr` "/Game/Maps/AlphaDemo/AlphaStageSelect.AlphaStageSelect"))

(event `/Game/Blueprint/Interface/Behivour/BPI_Common_Behaviour.Damaged`
  (params (KnockBack :type "Vector Structure") (Damage :type Integer) (HitParticle :type "NiagaraComponent Object Reference") (HitParticleScale :type "Float (double-precision)"))
  ; 피격 시
  (`/Game/Blueprint/Interface/BPI_IEnemyStateMachine.ChangeState` (`self.AC_DurahanStateMachine`) null)
  (`self.KnockBack` KnockBack)
  (bind _aswb_damage_display (cast `/Game/Blueprint/UI/Damage/WB_DamageDisplay` (`WidgetComponent.GetUserWidgetObject` (`self.Widget`))))
  (`/Game/Blueprint/UI/Damage/WB_DamageDisplay.DisplayDamage` _aswb_damage_display (`KismetMathLibrary.Conv_IntToInt64` Damage))
  (`self.PlayHitEffect` "/Game/VFX/SlashHitVFX/NS/NS_Hit_Halberd.NS_Hit_Halberd" 5.0))

(event `/Game/Blueprint/Interface/BPI_ShowVFX.PasteDecal`
  ; Comment
  (`self.PlayDecal`))

(fn `CheckPlayerInNormalAttackRange`
  (returns (`Player In Attack Range` :type Boolean))
  (return (`KismetArrayLibrary.Array_IsNotEmpty` (`PrimitiveComponent.GetOverlappingActors` (`self.NomalAttackRangeSphere`) "/Game/Blueprint/BP_ZZZ_AgentBase.BP_ZZZ_AgentBase_C"))))

(fn `GetAttackDetectBox`
  (returns (Box :type "BoxComponent Object Reference"))
  (return (`self.AttackDetectBox`)))

(fn `GetMesh`
  (returns (`Mesh Comp` :type "MeshComponent Object Reference"))
  (return (`self.Mesh`)))

(fn `PlayDecal`
  (bind _mesh (`self.Mesh`))
  (`NiagaraFunctionLibrary.SpawnSystemAttached` null _mesh "None" (`SkeletalMeshSocket.GetSocketLocation` (`.ReturnValue` (`SkinnedAsset.FindSocketInfo` (`SkinnedMeshComponent.SkinnedAsset` _mesh) "DecalSocket")) null) (struct) "KeepRelativeOffset" true))

(fn `UserConstructionScript`)