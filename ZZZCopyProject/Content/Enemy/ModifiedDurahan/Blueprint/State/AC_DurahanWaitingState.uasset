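; AC_DurahanWaitingState is the waiting state component in the Durahan boss's state machine.
; On BeginPlay it casts its owner to BP_Boss and caches it.
; Entering the state clears the boss's walking flag and starts a short timer, which then switches the boss's state machine to the walk state.
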(event `self.ReceiveBeginPlay`
  ; Comment
  (bind _asbp_boss (cast `/Game/Enemy/ModifiedDurahan/Blueprint/BP_Boss` (`self.GetOwner`)))
  (set `self.OwnerEnemy` _asbp_boss))

(event `/Game/Blueprint/Interface/BPI_IEnemyState.Enter`
  ; Comment
  (set `/Game/Enemy/ModifiedDurahan/Blueprint/BP_Boss.IsWalking` false (`self.OwnerEnemy`))
  (`KismetSystemLibrary.K2_SetTimerDelegate` (delegate `WaitingEnd`) 1.0))

(event `WaitingEnd`
  (bind _ownerenemy (`self.OwnerEnemy`))
  ; Comment
  (`/Game/Blueprint/Interface/BPI_IEnemyStateMachine.ChangeState` (`/Game/Enemy/ModifiedDurahan/Blueprint/BP_Boss.AC_DurahanStateMachine` _ownerenemy) (`/Game/Enemy/ModifiedDurahan/Blueprint/BP_Boss.AC_DurahanWalkState` _ownerenemy)))