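; Walk state component for the Durahan boss enemy's state machine, driving its movement until the player is within normal attack range.
; It caches its owner as BP_Boss on BeginPlay and toggles that boss's IsWalking flag on Enter and Exit.
; Each Update turns and walks the boss, or switches to the idle state and prints a debug string once the range check passes.
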(event `self.ReceiveBeginPlay`
  ; Comment
  (bind _asbp_boss (cast `/Game/Enemy/ModifiedDurahan/Blueprint/BP_Boss` (`self.GetOwner`)))
  (set `self.OwnerEnemy` _asbp_boss))

(event `/Game/Blueprint/Interface/BPI_IEnemyState.Update`
  (bind _ownerenemy (`self.OwnerEnemy`))
  (if (`/Game/Blueprint/BP_ZZZ_EnemyBase.CheckPlayerInNormalAttackRange` (`self.OwnerEnemy`))
    ; Comment
    (`/Game/Blueprint/Interface/BPI_IEnemyStateMachine.ChangeState` (`/Game/Enemy/ModifiedDurahan/Blueprint/BP_Boss.AC_DurahanStateMachine` _ownerenemy) (`/Game/Enemy/ModifiedDurahan/Blueprint/BP_Boss.AC_DurahanIdleState` _ownerenemy))
    (`KismetSystemLibrary.PrintString` "Hello")
    (else
      ; Comment
      (`/Game/Blueprint/BP_ZZZ_EnemyBase.Turn` (`self.OwnerEnemy`))
      (`/Game/Blueprint/BP_ZZZ_EnemyBase.Walk` (`self.OwnerEnemy`)))))

(event `/Game/Blueprint/Interface/BPI_IEnemyState.Enter`
  (set `/Game/Enemy/ModifiedDurahan/Blueprint/BP_Boss.IsWalking` true (`self.OwnerEnemy`)))

(event `/Game/Blueprint/Interface/BPI_IEnemyState.Exit`
  (set `/Game/Enemy/ModifiedDurahan/Blueprint/BP_Boss.IsWalking` false (`self.OwnerEnemy`)))