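; Actor component that runs the state machine for the Durahan boss, cached from its owning BP_Boss.
; ChangeState, skipped when the boss is dead, exits the current interface-based state, records it as previous and enters the requested one.
; With no valid current state, it ignores the request and enters the boss's idle state.
; Execute forwards updates to the current state.
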(event `self.ReceiveBeginPlay`
  ; Comment
  (bind _asbp_boss (cast `/Game/Enemy/ModifiedDurahan/Blueprint/BP_Boss` (`self.GetOwner`)))
  (set `self.OwnerEnemy` _asbp_boss))

(event `/Game/Blueprint/Interface/BPI_IEnemyStateMachine.ChangeState`
  (params (ChangeEnemyState :type "/Game/Blueprint/Interface/BPI_IEnemyState Interface"))
  (bind _currentstate (`self.CurrentState`))
  (if (not (`/Game/Blueprint/BP_ZZZ_CharacterBase.Dead?` (`self.OwnerEnemy`)))
    (if (`KismetSystemLibrary.IsValidInterface` (`self.CurrentState`))
      ; Comment
      (`/Game/Blueprint/Interface/BPI_IEnemyState.Exit` _currentstate)
      (set `self.PreviousState` _currentstate)
      (bind _output_get (set `self.CurrentState` ChangeEnemyState))
      (`/Game/Blueprint/Interface/BPI_IEnemyState.Enter` _output_get)
      (else
        ; 최초 실행
        (bind _output_get_2 (set `self.CurrentState` (`/Game/Enemy/ModifiedDurahan/Blueprint/BP_Boss.AC_DurahanIdleState` (`self.OwnerEnemy`))))
        (bind _output_get_3 (set `self.PreviousState` _output_get_2))
        (`/Game/Blueprint/Interface/BPI_IEnemyState.Enter` _output_get_3)))))

(event `/Game/Blueprint/Interface/BPI_IEnemyStateMachine.Execute`
  (bind _currentstate (`self.CurrentState`))
  ; Comment
  (if (`KismetSystemLibrary.IsValidInterface` _currentstate)
    (`/Game/Blueprint/Interface/BPI_IEnemyState.Update` _currentstate)))