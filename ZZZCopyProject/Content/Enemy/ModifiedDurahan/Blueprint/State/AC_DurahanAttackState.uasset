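; Actor component that serves as the attack state for the Durahan boss enemy's state machine.
; On begin play it caches its owner as a BP_Boss.
; On Enter it turns the boss, plays the attack montage on its mesh, and switches the state machine to the waiting state when the montage completes.
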(event `self.ReceiveBeginPlay`
  (bind _asbp_boss (cast `/Game/Enemy/ModifiedDurahan/Blueprint/BP_Boss` (`self.GetOwner`)))
  (set `self.OwnerEnemy` _asbp_boss))

(event `/Game/Blueprint/Interface/BPI_IEnemyState.Enter`
  (bind _ownerenemy (`self.OwnerEnemy`))
  (bind _ownerenemy_2 (`self.OwnerEnemy`))
  (`/Game/Blueprint/BP_ZZZ_EnemyBase.Turn` _ownerenemy_2)
  (`|PlayMontage` (`Character.Mesh` _ownerenemy_2) "/Game/Enemy/ModifiedDurahan/Animation/AM_Attack.AM_Attack"
    (:`OnCompleted`
      (`/Game/Blueprint/Interface/BPI_IEnemyStateMachine.ChangeState` (`/Game/Enemy/ModifiedDurahan/Blueprint/BP_Boss.AC_DurahanStateMachine` _ownerenemy) (`/Game/Enemy/ModifiedDurahan/Blueprint/BP_Boss.AC_DurahanWaitingState` _ownerenemy)))))