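; AC_DurahanDeadState is the death state component for the Durahan boss, caching its BP_Boss owner on BeginPlay.
; Entering the state flags the boss as dead and starts the AM_BossDie montage on its mesh.
; Without waiting for the montage to finish, it sets the capsule to ignore Pawn collision, then destroys the boss after a fixed delay.
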(event `self.ReceiveBeginPlay`
  ; Comment
  (bind _asbp_boss (cast `/Game/Enemy/ModifiedDurahan/Blueprint/BP_Boss` (`self.GetOwner`)))
  (set `self.OwnerEnemy` _asbp_boss))

(event `/Game/Blueprint/Interface/BPI_IEnemyState.Enter`
  (bind _ownerenemy (`self.OwnerEnemy`))
  ; Comment
  (set `/Game/Blueprint/BP_ZZZ_CharacterBase.Dead?` true _ownerenemy)
  (`|PlayMontage` (`Character.Mesh` _ownerenemy) "/Game/Enemy/ModifiedDurahan/Animation/AM_BossDie.AM_BossDie"
    (:`then`
      (`PrimitiveComponent.SetCollisionResponseToChannel` (`Character.CapsuleComponent` (`self.OwnerEnemy`)) "ECC_Pawn" "ECR_Ignore")
      (`KismetSystemLibrary.Delay` 5.0)
      (`Actor.K2_DestroyActor` (`self.OwnerEnemy`)))))