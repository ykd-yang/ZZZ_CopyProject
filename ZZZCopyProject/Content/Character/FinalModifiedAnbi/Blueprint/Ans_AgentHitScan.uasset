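; Anim notify state that runs Anbi's melee hit window during attack animations, with semi-auto targeting.
; On begin, it turns Anbi toward the first BP_Monster overlapping the TargetBox and resets the hit flag.
; Each tick, it polls AttackCollider overlaps and damages the monsters found by a fixed amount.
; IsAbleHitEnemy, set true after the first hit despite its name, limits damage to one pass per window.
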(fn `Received_NotifyBegin`
  (params (MeshComp :type "SkeletalMeshComponent Object Reference") (Animation :type "AnimSequenceBase Object Reference") (TotalDuration :type "Float (single-precision)") (EventReference :type "AnimNotifyEventReference Structure (by ref)"))
  (returns (ReturnValue :type Boolean))
  (locals (Player :type "/Game/Character/FinalModifiedAnbi/Blueprint/BP_Anbi Object Reference"))
  (bind _player (`local.Player`))
  ; 로컬 변수 설정
  (bind _asbp_anbi (cast `/Game/Character/FinalModifiedAnbi/Blueprint/BP_Anbi` (`ActorComponent.GetOwner` MeshComp)))
  (set `local.Player` _asbp_anbi)
  (bind _overlappingactors (`PrimitiveComponent.GetOverlappingActors` (`/Game/Character/FinalModifiedAnbi/Blueprint/BP_Anbi.TargetBox` _asbp_anbi) "/Game/Monster/BP_Monster.BP_Monster_C"))
  (if (not (`KismetArrayLibrary.Array_IsEmpty` _overlappingactors))
    ; 세미 오토 타겟팅 시스템
    (`Actor.K2_SetActorRotation` _player (`KismetMathLibrary.FindLookAtRotation` (`Actor.K2_GetActorLocation` _player) (`Actor.K2_GetActorLocation` (`|GetArrayItem` _overlappingactors))) false))
  (set `/Game/Character/FinalModifiedAnbi/Blueprint/BP_Anbi.IsAbleHitEnemy` false (`local.Player`))
  (return false))

(fn `Received_NotifyEnd`
  (params (MeshComp :type "SkeletalMeshComponent Object Reference") (Animation :type "AnimSequenceBase Object Reference") (EventReference :type "AnimNotifyEventReference Structure (by ref)"))
  (returns (ReturnValue :type Boolean))
  (return false))

(fn `Received_NotifyTick`
  (params (MeshComp :type "SkeletalMeshComponent Object Reference") (Animation :type "AnimSequenceBase Object Reference") (FrameDeltaTime :type "Float (single-precision)") (EventReference :type "AnimNotifyEventReference Structure (by ref)"))
  (returns (ReturnValue :type Boolean))
  (locals (Anby :type "/Game/Character/FinalModifiedAnbi/Blueprint/BP_Anbi Object Reference"))
  (bind _anby (`local.Anby`))
  (bind _overlappingactors (`PrimitiveComponent.GetOverlappingActors` (`/Game/Character/FinalModifiedAnbi/Blueprint/BP_Anbi.Attack Collider` _anby) "/Game/Monster/BP_Monster.BP_Monster_C"))
  ; 지역 변수 설정
  (bind _asbp_anbi (cast `/Game/Character/FinalModifiedAnbi/Blueprint/BP_Anbi` (`ActorComponent.GetOwner` MeshComp)))
  (set `local.Anby` _asbp_anbi)
  ; 공격 당 1회만 데미지 부여
  (if (not (`/Game/Character/FinalModifiedAnbi/Blueprint/BP_Anbi.IsAbleHitEnemy` _anby))
    ; 명중한 적에게 데미지
    (if (not (`KismetArrayLibrary.Array_IsEmpty` _overlappingactors))
      (for _array_element _overlappingactors
        (bind _asbp_monster (cast `/Game/Monster/BP_Monster` _array_element))
        (`/Game/Monster/BP_Monster.TakeDamage` _asbp_monster 10.0 (`local.Anby`)))
      ; 더 이상 적에게 데미지 부여 없음
      (set `/Game/Character/FinalModifiedAnbi/Blueprint/BP_Anbi.IsAbleHitEnemy` true (`local.Anby`))
      (return false))))