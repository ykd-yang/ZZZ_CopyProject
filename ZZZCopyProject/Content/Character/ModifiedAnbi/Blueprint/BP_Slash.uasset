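; Short-lived slash attack actor for the Anbi character that applies hits to enemies within its box.
; Spawn plays a scaled katana Niagara effect at the actor's transform, starts a looping HitScan timer and destroys the actor after a brief delay.
; HitScan polls the box for overlapping enemies and uses HitMap to call each one's hit event only once, passing Anbi.
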(event `Spawn`
  (params (Anbi :type "/Game/Character/ModifiedAnbi/Blueprint/BP_Anbi Object Reference"))
  (bind (_returnvalue_location _returnvalue_rotation) (`KismetMathLibrary.BreakTransform` (`self.GetTransform`)))
  (bind _returnvalue (`NiagaraFunctionLibrary.SpawnSystemAtLocation` "/Game/VFX/SlashHitVFX/NS/NS_Slash_Katana.NS_Slash_Katana" _returnvalue_location _returnvalue_rotation))
  (`SceneComponent.SetWorldScale3D` _returnvalue (1.5 1.5 1.5))
  (`KismetSystemLibrary.K2_SetTimerDelegate` (delegate `HitScan`) 0.1 true)
  (`KismetSystemLibrary.Delay` 0.5)
  (`self.K2_DestroyActor`))

(event `HitScan`
  (bind _overlappingactors (`PrimitiveComponent.GetOverlappingActors` (`self.Box`) "/Game/Blueprint/BP_ZZZ_EnemyBase.BP_ZZZ_EnemyBase_C"))
  (if (`KismetArrayLibrary.Array_IsNotEmpty` _overlappingactors)
    (for _array_element _overlappingactors
      (bind _asbp_zzz_enemy_base (cast `/Game/Blueprint/BP_ZZZ_EnemyBase` _array_element))
      (if (not (`BlueprintMapLibrary.Map_Contains` (`self.HitMap`) _asbp_zzz_enemy_base))
        (`BlueprintMapLibrary.Map_Add` (`self.HitMap`) _asbp_zzz_enemy_base true)
        (`/Game/Blueprint/BP_ZZZ_CharacterBase.OnCharacterHItEvent` _asbp_zzz_enemy_base (stale `Spawn` Anbi))))))

(fn `UserConstructionScript`)