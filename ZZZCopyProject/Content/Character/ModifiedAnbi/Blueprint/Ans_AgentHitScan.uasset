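; Anim notify state for BP_Anbi's attacks that handles semi-auto targeting and hit detection.
; On begin it arms the hit flag and snaps Anbi's rotation toward the nearest living character in TargetBox that passes the IFF check.
; On tick, while armed, it sends the hit event to every enemy overlapping AttackCollider, then clears the flag, so damage is checked only once per notify window.
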(fn `Received_NotifyBegin`
  (params (MeshComp :type "SkeletalMeshComponent Object Reference") (Animation :type "AnimSequenceBase Object Reference") (TotalDuration :type "Float (single-precision)") (EventReference :type "AnimNotifyEventReference Structure (by ref)"))
  (returns (ReturnValue :type Boolean))
  (locals (Player :type "/Game/Character/ModifiedAnbi/Blueprint/BP_Anbi Object Reference") (ClosestEnemy :type "/Game/Blueprint/BP_ZZZ_CharacterBase Object Reference") (ClosestDistance :type "Float (double-precision)" :default 100000.0))
  (bind _player (`local.Player`))
  ; 로컬 변수 설정
  (bind _asbp_anbi (cast `/Game/Character/ModifiedAnbi/Blueprint/BP_Anbi` (`ActorComponent.GetOwner` MeshComp)))
  (bind _output_get (set `local.Player` _asbp_anbi))
  ; 세미 오토 타겟팅 시스템
  (set `/Game/Character/ModifiedAnbi/Blueprint/BP_Anbi.IsAbleHitEnemy` true _output_get)
  (bind _overlappingactors (`PrimitiveComponent.GetOverlappingActors` (`/Game/Character/ModifiedAnbi/Blueprint/BP_Anbi.TargetBox` _output_get) "/Game/Blueprint/BP_ZZZ_CharacterBase.BP_ZZZ_CharacterBase_C"))
  (if (not (`KismetArrayLibrary.Array_IsEmpty` _overlappingactors))
    (for _array_element _overlappingactors
      (bind _asbp_zzz_character_base (cast `/Game/Blueprint/BP_ZZZ_CharacterBase` _array_element))
      (bind _returnvalue (`KismetMathLibrary.Vector_Distance` (`Actor.K2_GetActorLocation` _array_element) (`Actor.K2_GetActorLocation` (`local.Player`))))
      (if (and (`|EnumEquality` (`/Game/Blueprint/BP_ZZZ_CharacterBase.IFF` _asbp_zzz_character_base) "NewEnumerator1") (not (`/Game/Blueprint/BP_ZZZ_CharacterBase.Dead?` _asbp_zzz_character_base)) (> (`local.ClosestDistance`) _returnvalue))
        (set `local.ClosestDistance` _returnvalue)
        (set `local.ClosestEnemy` _asbp_zzz_character_base)))
    ; 가장 가까운 목표로 회전
    (`/Engine/EditorBlueprintResources/StandardMacros.IsValid` (`local.ClosestEnemy`)
      (:`Is Valid`
        (`Actor.K2_SetActorRotation` (`local.Player`) (`KismetMathLibrary.FindLookAtRotation` (`Actor.K2_GetActorLocation` (`local.Player`)) (`Actor.K2_GetActorLocation` (`local.ClosestEnemy`))) false)
        (set `/Game/Character/ModifiedAnbi/Blueprint/BP_Anbi.IsAbleHitEnemy` true _player)
        (`KismetSystemLibrary.PrintString` null (`KismetStringLibrary.Concat_StrStr` (`KismetSystemLibrary.GetDisplayName` _player) "Execute SemiAutoTargeting!") true true (struct :`G` 1.0 :`A` 1.0))
        (return false)))))

(fn `Received_NotifyEnd`
  (params (MeshComp :type "SkeletalMeshComponent Object Reference") (Animation :type "AnimSequenceBase Object Reference") (EventReference :type "AnimNotifyEventReference Structure (by ref)"))
  (returns (ReturnValue :type Boolean))
  (return false))

(fn `Received_NotifyTick`
  (params (MeshComp :type "SkeletalMeshComponent Object Reference") (Animation :type "AnimSequenceBase Object Reference") (FrameDeltaTime :type "Float (single-precision)") (EventReference :type "AnimNotifyEventReference Structure (by ref)"))
  (returns (ReturnValue :type Boolean))
  (locals (Anby :type "/Game/Character/ModifiedAnbi/Blueprint/BP_Anbi Object Reference"))
  ; 지역 변수 설정
  (bind _asbp_anbi (cast `/Game/Character/ModifiedAnbi/Blueprint/BP_Anbi` (`ActorComponent.GetOwner` MeshComp)))
  (set `local.Anby` _asbp_anbi)
  ; 공격 당 1회만 데미지 부여
  (if (`/Game/Character/ModifiedAnbi/Blueprint/BP_Anbi.IsAbleHitEnemy` (`local.Anby`))
    ; 명중한 적에게 데미지
    (for _array_element (`PrimitiveComponent.GetOverlappingActors` (`/Game/Character/ModifiedAnbi/Blueprint/BP_Anbi.Attack Collider` (`local.Anby`)) "/Game/Blueprint/BP_ZZZ_EnemyBase.BP_ZZZ_EnemyBase_C")
      (bind _asbp_zzz_character_base (cast `/Game/Blueprint/BP_ZZZ_CharacterBase` _array_element))
      (`/Game/Blueprint/BP_ZZZ_CharacterBase.OnCharacterHItEvent` _asbp_zzz_character_base (`local.Anby`)))
    ; 더 이상 적에게 데미지 부여 없음
    (set `/Game/Character/ModifiedAnbi/Blueprint/BP_Anbi.IsAbleHitEnemy` false (`local.Anby`))
    (return false)))