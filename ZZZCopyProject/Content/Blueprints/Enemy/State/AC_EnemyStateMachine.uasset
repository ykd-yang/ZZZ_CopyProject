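; AC_EnemyStateMachine is a component that runs the state machine for a BP_Enemy owner, cached on BeginPlay.
; ChangeState exits the current interface-based state and enters the requested one; with no valid current state, it enters the enemy's Idle state instead, ignoring the request.
; Execute forwards to the current state's Update.
; PreviousState is assigned after each switch, so it mirrors the new state rather than the old one.
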(event `self.ReceiveBeginPlay`
  (bind _asbp_enemy (cast `/Game/Blueprints/Enemy/State/BP_Enemy` (`self.GetOwner`)))
  (set `self.OwnerEnemy` _asbp_enemy)
  (`KismetSystemLibrary.PrintString` (`KismetSystemLibrary.GetDisplayName` _asbp_enemy)))

(event `/Game/Interfaces/BPI_IEnemyStateMachine.ChangeState`
  (params (ChangeEnemyState :type "/Game/Interfaces/BPI_IEnemyState Interface"))
  (bind _currentstate (`self.CurrentState`))
  (if (`KismetSystemLibrary.IsValidInterface` (`self.CurrentState`))
    (`/Game/Interfaces/BPI_IEnemyState.Exit` _currentstate)
    (bind _output_get (set `self.CurrentState` ChangeEnemyState))
    (`/Game/Interfaces/BPI_IEnemyState.Enter` _output_get)
    (set `self.PreviousState` _currentstate)
    (else
      (bind _output_get_2 (set `self.CurrentState` (`/Game/Blueprints/Enemy/State/BP_Enemy.AC_EnemyIdleState` (`self.OwnerEnemy`))))
      (set `self.PreviousState` _output_get_2)
      (`/Game/Interfaces/BPI_IEnemyState.Enter` (`self.CurrentState`)))))

(event `/Game/Interfaces/BPI_IEnemyStateMachine.Execute`
  (bind _currentstate (`self.CurrentState`))
  (if (`KismetSystemLibrary.IsValidInterface` _currentstate)
    (`/Game/Interfaces/BPI_IEnemyState.Update` _currentstate)))