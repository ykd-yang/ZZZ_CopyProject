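; Enemy idle state component for the enemy state machine, cached against its owning BP_Enemy on BeginPlay.
; Entering clears the owner's IsWalking flag, and both Enter and Exit print debug messages.
; Each Update calls the owner's CheckDistanceWithPlayer and switches to the attack state if it returns true, otherwise to the walk state, so idle transitions out on its first update.
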(event `self.ReceiveBeginPlay`
  (bind _asbp_enemy (cast `/Game/Blueprints/Enemy/State/BP_Enemy` (`self.GetOwner`)))
  (set `self.OwnerEnemy` _asbp_enemy))

(event `/Game/Interfaces/BPI_IEnemyState.Enter`
  (set `/Game/Blueprints/Enemy/State/BP_Enemy.isWalking?` false (`self.OwnerEnemy`))
  (`KismetSystemLibrary.PrintString` "아이들 진입"))

(event `/Game/Interfaces/BPI_IEnemyState.Exit`
  (`KismetSystemLibrary.PrintString` "아이들 나감"))

(event `/Game/Interfaces/BPI_IEnemyState.Update`
  (bind _ownerenemy (`self.OwnerEnemy`))
  (bind _ac_enemystatemachine (`/Game/Blueprints/Enemy/State/BP_Enemy.AC_EnemyStateMachine` _ownerenemy))
  (bind _canattackdistance (`/Game/Blueprints/Enemy/State/BP_Enemy.CheckDistanceWithPlayer` (`self.OwnerEnemy`)))
  (if _canattackdistance
    (`/Game/Interfaces/BPI_IEnemyStateMachine.ChangeState` _ac_enemystatemachine (`/Game/Blueprints/Enemy/State/BP_Enemy.AC_EnemyAttackState` _ownerenemy))
    (else
      (`/Game/Interfaces/BPI_IEnemyStateMachine.ChangeState` _ac_enemystatemachine (`/Game/Blueprints/Enemy/State/BP_Enemy.AC_EnemyWalkState` _ownerenemy)))))