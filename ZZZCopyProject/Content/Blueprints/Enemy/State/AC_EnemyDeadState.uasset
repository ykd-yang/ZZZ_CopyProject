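; AC_EnemyDeadState is an enemy state component that handles the death of a BP_Enemy owner.
; On Enter it caches the owner and starts the death montage on its mesh.
; After a fixed delay, not tied to montage completion, it adds a kill to BP_AlphaManager and destroys the enemy.
; Update and Exit are empty.
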(event `self.ReceiveBeginPlay`
  (bind _asbp_enemy (cast `/Game/Blueprints/Enemy/State/BP_Enemy` (`self.GetOwner`)))
  (set `self.OwnerEnemy` _asbp_enemy))

(event `/Game/Interfaces/BPI_IEnemyState.Exit`)

(event `/Game/Interfaces/BPI_IEnemyState.Update`)

(event `/Game/Interfaces/BPI_IEnemyState.Enter`
  (bind _returnvalue (`self.GetOwner`))
  (bind _asbp_enemy (cast `/Game/Blueprints/Enemy/State/BP_Enemy` _returnvalue))
  (bind _output_get (set `self.OwnerEnemy` _asbp_enemy))
  (`|PlayMontage` (`Character.Mesh` _output_get) "/Game/Enemy/ModifiedClaymore/Animation/Montage/AM_EnemyDie.AM_EnemyDie"
    (:`then`
      (`KismetSystemLibrary.Delay` 2.0)
      (bind _returnvalue_2 (`GameplayStatics.GetActorOfClass` "/Game/Blueprints/BP_AlphaManager.BP_AlphaManager_C"))
      (`/Game/Blueprints/BP_AlphaManager.AddKillCount` _returnvalue_2)
      (`Actor.K2_DestroyActor` _returnvalue))))