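; Enemy Blueprint that moves toward, turns to and reacts to damage from the player pawn, driven by a state machine component.
; BeginPlay enters Idle, Tick runs the machine once spawning ends, and death switches to Dead.
; Helpers provide direct location-based walking and yaw targeting, gated by collider overlap and a dot-product FOV check without arccosine.
; Damage fires the character hit event and displays player ATK in a widget.
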(event `self.ReceiveBeginPlay`
  (bind _asbp_zzz_agent_base (cast `/Game/Blueprints/BP_ZZZ_AgentBase` (`GameplayStatics.GetPlayerPawn` 0)))
  (set `self.Player` _asbp_zzz_agent_base)
  (`/Game/Interfaces/BPI_IEnemyStateMachine.ChangeState` (`self.AC_EnemyStateMachine`) (`self.AC_EnemyIdleState`)))

(event `self.ReceiveTick`
  (params (DeltaSeconds :type "Float (single-precision)"))
  (if (`self.EndSpawn`)
    (`/Game/Interfaces/BPI_IEnemyStateMachine.Execute` (`self.AC_EnemyStateMachine`))))

(event `/Game/Blueprints/BPI_Behaivour.PlayDeath`
  (`self.Die`))

(event `/Game/Blueprints/BPI_Behaivour.GetHit`
  (`|PlayMontage` (`self.Mesh`) "/Game/Enemy/ModifiedClaymore/Animation/Montage/AM_EnemyHit.AM_EnemyHit"))

(fn `AttackTargeting`
  (bind _infov (`self.CheckFov`))
  (if _infov
    (`self.Turn`)))

(fn `CheckDistanceWithPlayer`
  (returns (CanAttackDistance :type Boolean))
  (if (`KismetArrayLibrary.Array_IsNotEmpty` (`PrimitiveComponent.GetOverlappingActors` (`self.AttackDetectCollider`) "/Game/Blueprints/BP_ZZZ_AgentBase.BP_ZZZ_AgentBase_C"))
    (return true)
    (else
      (return false))))

(fn `CheckFov`
  (returns (InFov :type Boolean))
  (bind _canattackdistance (`self.CheckDistanceWithPlayer`))
  (return (and (<= (`KismetMathLibrary.RadiansToDegrees` (`KismetMathLibrary.Dot_VectorVector` (`KismetMathLibrary.Normal` (- (`self.K2_GetActorLocation` (`self.Player`)) (`self.K2_GetActorLocation` self))) (`KismetMathLibrary.Normal` (`self.GetActorForwardVector` self)))) (`self.FovAngle`)) _canattackdistance)))

(fn `Die`
  (`/Game/Interfaces/BPI_IEnemyStateMachine.ChangeState` (`self.AC_EnemyStateMachine`) (`self.AC_EnemyDeadState`)))

(fn `TakeDamage`
  (locals (EnemyOwner :type "/Game/Blueprints/BP_ZZZ_CharacterBase Object Reference"))
  (bind _player (`self.Player`))
  (`KismetSystemLibrary.PrintString` "데미지 호출")
  (bind _asbp_zzz_character_base (cast `/Game/Blueprints/BP_ZZZ_CharacterBase` self))
  ; 01. 죽었는지 검사
  (set `local.EnemyOwner` _asbp_zzz_character_base)
  (if (not (`/Game/Blueprints/BP_ZZZ_CharacterBase.IsDead?` _asbp_zzz_character_base))
    (`self.OnCharacterHItEvent` (`local.EnemyOwner`) _player)
    (bind _aswb_damage_display (cast `/Game/Blueprints/UI/WB_DamageDisplay` (`WidgetComponent.GetUserWidgetObject` (`self.Widget`))))
    (`/Game/Blueprints/UI/WB_DamageDisplay.DisplayDamage` _aswb_damage_display (`KismetMathLibrary.Conv_IntToInt64` (`/Game/Blueprints/BP_ZZZ_CharacterBase.ATK` _player)))))

(fn `Turn`
  (bind (_returnvalue_x _returnvalue_y) (`KismetMathLibrary.BreakVector` (- (`self.K2_GetActorLocation` (`self.Player`)) (`self.K2_GetActorLocation`))))
  (`self.K2_SetActorRotation` (`KismetMathLibrary.MakeRotator` 0.0 0.0 (`KismetMathLibrary.RadiansToDegrees` (`KismetMathLibrary.Atan2` _returnvalue_y _returnvalue_x))))
  (return))

(fn `UserConstructionScript`)

(fn `Walking`
  (locals (Dir :type "Vector Structure" :default (0.0 0.0 0.0)))
  (bind _output_get (set `local.Dir` (`KismetMathLibrary.Normal` (- (`self.K2_GetActorLocation` (`self.Player`)) (`self.K2_GetActorLocation`)))))
  (`self.K2_SetActorLocation` (+ (* (* (`self.Speed`) (`GameplayStatics.GetWorldDeltaSeconds`)) _output_get) (`self.K2_GetActorLocation`))))