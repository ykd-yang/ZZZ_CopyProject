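; Base character Blueprint that applies incoming damage to HP when its hit event receives another actor.
; Hits from Enemy or Neutral characters, identified by IFF, deal the attacker's ATK reduced by this character's DEF as a percentage.
; Hits from traps subtract the trap's DMG directly, ignoring DEF.
; Both paths clamp and truncate HP and print a debug message, with no death handling here.
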(event Custom|OnCharacterHItEvent
  (params (other :type Actor%20Object%20Reference))
  (Utilities|FlowControl|Sequence
    (:then_0
      ;[0.15 0.15 0.15 0.5] 공격 유형을 확인한 후 데미지 적용
      (bind _asbp_zzz_character_base (Utilities|Casting|CastToBP_ZZZ_CharacterBase other))
      (switch Utilities|FlowControl|Switch|SwitchonTeamType (Variables|BP_ZZZ_CharacterBase_C|GetIFF _asbp_zzz_character_base)
        (:NewEnumerator1
          _)
        (:NewEnumerator2
          _))
      (Variables|Default|SetHP (Math|Float|Truncate (Math|Float|Clamp(Float) (- (Variables|Default|GetHP) (|(((100-defend)/100)*attack) (Math|Conversions|ToFloat(Integer) (Variables|Default|GetDEF)) (Math|Conversions|ToFloat(Integer) (Variables|BP_ZZZ_CharacterBase_C|GetATK _asbp_zzz_character_base)))) 0.0 1e+05)))
      (Development|PrintString "AgentDamaged"))
    (:then_1
      ;[0.15 0.15 0.15 0.5] 함정 데미지 적용
      (bind _asbp_zzz_trap_base (Utilities|Casting|CastToBP_ZZZ_TrapBase other))
      (Variables|Default|SetHP (Math|Float|Truncate (Math|Float|Clamp(Float) (Math|Conversions|ToFloat(Integer) (- (Variables|Default|GetHP) (Variables|/Game/Blueprints/BP_ZZZ_TrapBase.BP_ZZZ_TrapBase_C|GetDMG _asbp_zzz_trap_base))) 0.0 1e+05)))
      (Development|PrintString "AgentDamaged"))))

(event EventBeginPlay)

(event Collision|EventActorBeginOverlap
  (params (OtherActor :type Actor%20Object%20Reference)))

(event EventTick
  (params (DeltaSeconds :type Float%20%28single-precision%29)))

(fn ConstructionScript)