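; BP_AlphaManager is a level manager actor that counts kills and triggers the boss encounter.
; BeginPlay caches the player pawn as a BP_ZZZ_AgentBase reference.
; Each AddKillCount call increments KillCount; when the count hits the threshold, it waits briefly, teleports the player to SpawbLocation, then sets EndSpawn on the BP_Boss found in the level after a short delay.
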(event `self.ReceiveBeginPlay`
  (bind _asbp_zzz_agent_base (cast `/Game/Blueprints/BP_ZZZ_AgentBase` (`GameplayStatics.GetPlayerPawn` 0)))
  (set `self.Player` _asbp_zzz_agent_base))

(event `AddKillCount`
  (bind _result (`/Engine/EditorBlueprintResources/StandardMacros.IncrementInt` (`self.KillCount`))
    (:`  `
      (if (== _result 3)
        (`KismetSystemLibrary.Delay` 2.0)
        (`self.K2_SetActorLocation` (`self.Player`) (`self.SpawbLocation`) false true)
        (bind _returnvalue (`GameplayStatics.GetActorOfClass` "/Game/Blueprints/Boss/BP_Boss.BP_Boss_C"))
        (`KismetSystemLibrary.Delay` 0.2)
        (set `/Game/Blueprints/Boss/BP_Boss.EndSpawn` true _returnvalue)))))

(fn `UserConstructionScript`)