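; BP_ZZZ_AgentBase is an agent character base handling automatic running, a charge-based dodge and hit filtering.
; Tick tracks velocity, starts a timer that raises walk speed after sustained movement, and refills dodge charges up to a cap.
; Right-click spends a charge to dash forward, or backward at low forward speed, with a timer restoring speed.
; Hit events pass to the character hit handler unless IsOnDodging is set.
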(event `OnAgentHitEvent`
  (params (other :type "/Game/Blueprints/BP_ZZZ_CharacterBase Object Reference"))
  (if (not (`self.IsOnDodging`))
    (`self.OnCharacterHItEvent` other)
    (`KismetSystemLibrary.PrintString` "맞아야지")))

(event `self.ReceiveTick`
  (params (DeltaSeconds :type "Float (single-precision)"))
  (`|ExecutionSequence`
    (:`then_0`
      ; 캐릭터 무브 컴포넌트를 사용하여 이동 상태를 확인 - 이동 상태로 전환하거나 정지 상태로 전환한다
      (if (> (`KismetMathLibrary.VSize` (`MovementComponent.Velocity` (`self.CharacterMovement`))) 10.0)
        (set `self.IsMoving` true)
        (else
          (set `self.IsMoving` false)
          (set `self.IsRunning` false)
          ;; 이동 속도 감소 및 달리기 전환 타이머 비활성
          (set `CharacterMovementComponent.MaxWalkSpeed` 600.0 (`self.CharacterMovement`))
          (`KismetSystemLibrary.K2_ClearAndInvalidateTimerHandle` (`self.RunningTransitionTimerHandle`)))))
    (:`then_1`
      ; Comment
      ;; 이동 상태인데 아직 달리는 상태는 아닌가 확인
      (if (and (`self.IsMoving`) (not (`self.IsRunning`)))
        ;; 달리기 시작 타이머 시작한다
        (if (not (`KismetSystemLibrary.K2_IsValidTimerHandle` (`self.RunningTransitionTimerHandle`)))
          (bind _returnvalue (`KismetSystemLibrary.K2_SetTimerDelegate` (delegate `EnterRunningState`) 3.0))
          (set `self.RunningTransitionTimerHandle` _returnvalue)
          (`KismetSystemLibrary.PrintString` "Running Timer Start"))))
    (:`then_2`
      (`self.DodgeChargingFuction` DeltaSeconds))))

(event `EnterRunningState`
  ; Comment
  ;; 달리기 시작 타이머가 발동 되면 이동 속도 증가
  (`KismetSystemLibrary.PrintString` "Enter Running State")
  (set `self.IsRunning` true)
  (set `CharacterMovementComponent.MaxWalkSpeed` 1000.0 (`self.CharacterMovement`))
  (`KismetSystemLibrary.K2_ClearAndInvalidateTimerHandle` (`self.RunningTransitionTimerHandle`)))

(event `Key|RightMouseButton`
  (params (Key :type "Key Structure"))
  (bind _charactermovement (`self.CharacterMovement`))
  ; 우클릭 회피 로직
  (:`Pressed`
    (if (>= (`self.Dodging Count`) 1)
      (set `self.IsRightMouseDown` true)
      (set `CharacterMovementComponent.MaxWalkSpeed` 1800.0 _charactermovement)
      (set `MovementComponent.Velocity` (* (`self.GetActorForwardVector`) (`KismetMathLibrary.SelectInt` -1800 1800 (<= (`KismetMathLibrary.Dot_VectorVector` (`self.GetVelocity`) (`self.GetActorForwardVector`)) 200.0))) _charactermovement)
      (`KismetSystemLibrary.K2_SetTimerDelegate` (delegate `DodgeOverEvent`) 0.4)
      (bind _output_get (set `self.Dodging Count` (- (`self.Dodging Count`) 1)))
      (`KismetSystemLibrary.PrintString` (`KismetStringLibrary.Conv_IntToString` _output_get))))
  (:`Released`
    (set `self.IsRightMouseDown` false)))

(event `DodgeOverEvent`
  ; 우클릭 회피 로직
  (set `CharacterMovementComponent.MaxWalkSpeed` 600.0 (`self.CharacterMovement`)))

(fn `DodgeChargingFuction`
  (params (NewParam :type "Float (double-precision)"))
  (if (not (>= (`self.Dodging Count`) 3))
    (bind _output_get (set `self.Current Time` (+ NewParam (`self.Current Time`))))
    (if (>= _output_get (`self.Dodging Cooltime`))
      (`/Engine/EditorBlueprintResources/StandardMacros.IncrementInt` (`self.Dodging Count`)
        (:`  `
          (set `self.Current Time` 0.0))))))

(fn `UserConstructionScript`)